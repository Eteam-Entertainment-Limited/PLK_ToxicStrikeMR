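; Player state for a shared-space mixed-reality VR shooter that runs the match alongside Oculus spatial-anchor sharing.
; Server RPCs and multicasts set the Oculus net ID, share anchors and align pawns to anchors.
; Kill thresholds clear levels and trigger quiz questions, then in the boss stage expose a weakpoint, where correct answers damage the boss.
; Coins, kills and items are tracked here; boss death shows graded results, while timeout drops a prison.
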(event `Spatial Anchor Begin`
  ;[1 1 1] Spatial anchor
  ;;[1 1 1] Wait for replication to get local player state
  (`KismetSystemLibrary.Delay` 2.0)
  (if (== (`Controller.PlayerState` (`GameplayStatics.GetPlayerController` 0)) self)
    ;;[1 1 1] Update the oculus net ID on the server
    (bind _returnvalue (`SharedAnchorsSampleBPLibrary.GetLocalPlayerOculusNetID`))
    (bind _output_get (set `self.OculusNetID` _returnvalue))
    (`self.Server_SetOculusNetID` _output_get)))

(event `Server_SetOculusNetID`
  (params (NetID :type String))
  ;[1 1 1] Spatial anchor
  (set `self.OculusNetID` NetID)
  (`self.NetMutlicast_NewPlayerJoined`))

(event `NetMutlicast_NewPlayerJoined`
  ;[1 1 1] Spatial anchor
  (bind _asbp_vrpawn (cast `/Game/PLK_MR/Blueprints/BP_VRPawn` (`GameplayStatics.GetPlayerPawn` 0)))
  (bind _spatialanchormanager_ac (`/Game/PLK_MR/Blueprints/BP_VRPawn.SpatialAnchorManager_AC` _asbp_vrpawn))
  (`/Game/PLK_MR/Blueprints/Components/BP_SpatialAnchorManagerComponent.ShareSpecifiedAnchors` _spatialanchormanager_ac (`/Game/PLK_MR/Blueprints/Components/BP_SpatialAnchorManagerComponent.SharedAnchors` _spatialanchormanager_ac)))

(event `Server_ShareIDs`
  (params (UUIDs :type "Array of OculusXRUUID Structure"))
  ;[1 1 1] Spatial anchor
  (`self.NetMutlicast_ShareAnchors` UUIDs))

(event `NetMutlicast_ShareAnchors`
  (params (UUIDs :type "Array of OculusXRUUID Structure"))
  (bind _returnvalue (`GameplayStatics.GetPlayerPawn` 0))
  (bind _returnvalue_2 (`self.GetComponentByClass` _returnvalue "/Game/PLK_MR/Blueprints/Components/BP_SpatialAnchorManagerComponent.BP_SpatialAnchorManagerComponent_C"))
  ;[1 1 1] Spatial anchor
  (`/Engine/EditorBlueprintResources/StandardMacros.IsValid` _returnvalue
    (:`Is Valid`
      (`/Engine/EditorBlueprintResources/StandardMacros.IsValid` _returnvalue_2
        (:`Is Valid`
          (`/Game/PLK_MR/Blueprints/Components/BP_SpatialAnchorManagerComponent.GetAllSharedAnchors` _returnvalue_2 UUIDs))))))

(event `Server_OrientToAnchor`
  (params (Position :type "Vector Structure") (Rotation :type "Rotator Structure"))
  (bind _pawnprivate (`self.PawnPrivate`))
  ;[1 1 1] Spatial anchor
  (`self.K2_SetActorLocation` _pawnprivate Position false true)
  (`self.K2_SetActorRotation` _pawnprivate Rotation true)
  (`self.NetMulticast_SetPosition` Position Rotation))

(event `NetMulticast_SetPosition`
  (params (Position :type "Vector Structure") (Rotation :type "Rotator Structure"))
  (bind _pawnprivate (`self.PawnPrivate`))
  ;[1 1 1] Spatial anchor
  (`self.K2_SetActorLocation` _pawnprivate Position false true)
  (`self.K2_SetActorRotation` _pawnprivate Rotation true))

(event `Server_SpawnCube`
  (params (Position :type "Vector Structure"))
  ;[1 1 1] Spatial anchor
  (`|SpawnActorFromClass` "/Game/PLK_MR/Blueprints/BP_Cube.BP_Cube_C" (`KismetMathLibrary.MakeTransform` Position (struct) (0.25 0.25 0.25)) "Undefined" "OverrideRootScale" null null))

(event `Losing`
  (bind (_returnvalue_x _returnvalue_y) (`KismetMathLibrary.BreakVector` (`SceneComponent.K2_GetComponentLocation` (`/Game/PLK_MR/Blueprints/BP_VRPawn.Camera` (`/Game/PLK_MR/Library/BP_FunctionLibrary.Get VR Pawn`)))))
  (if (`self.GameStarted`)
    (set `self.GameStarted` false)
    (`/Game/PLK_MR/Blueprints/BP_Room.StopSpawning` (`self.RoomRef`))
    (`self.DeleteAllEnemy`)
    (`/Game/PLK_MR/Blueprints/Components/BP_BGMController.ChangeMusic` (`/Game/PLK_MR/Blueprints/BP_VRPawn.BP_BGMController` (`/Game/PLK_MR/Library/BP_FunctionLibrary.Get VR Pawn`)) "NewEnumerator5")
    (`|ExecutionSequence`
      (:`then_0`
        (bind _outactors (`GameplayStatics.GetAllActorsOfClass` "/Game/PLK_MR/Blueprints/Gun/BP_Gun.BP_Gun_C"))
        (for _array_element _outactors
          (`/Game/PLK_MR/Blueprints/Gun/BP_Gun.Destroy` _array_element))
        (bind _outactors_2 (`GameplayStatics.GetAllActorsOfClass` "/Game/PLK_MR/Blueprints/BP_Chest.BP_Chest_C"))
        (for _array_element_2 _outactors_2
          (`self.K2_DestroyActor` _array_element_2))
        (`self.K2_DestroyActor` (`self.BossRef`)))
      (:`then_1`
        (`|SpawnActorFromClass` "/Game/PLK_MR/Blueprints/BP_Prison.BP_Prison_C" (`KismetMathLibrary.MakeTransform` (`KismetMathLibrary.MakeVector` _returnvalue_x _returnvalue_y)) "Undefined" "MultiplyWithRoot" null null)))))

(event `Server_ThrowCube`
  (params (Cube :type "/Game/PLK_MR/Blueprints/BP_Cube Object Reference"))
  ;[1 1 1] Spatial anchor
  (`/Game/PLK_MR/Blueprints/BP_Cube.Explode Cube` Cube))

(event `self.ReceiveBeginPlay`
  ;[1 1 1] Begin play
  (`|ExecutionSequence`
    (:`then_0`
      (`self.Spatial Anchor Begin`))
    (:`then_1`
      (bind _levels (`/Game/PLK_MR/Library/BP_FunctionLibrary.SetGameLevels` "NewEnumerator0"))
      (`self.Levels_Changing` _levels))
    (:`then_2`
      (bind _returnvalue (`GameplayStatics.GetActorOfClass` "/Game/PLK_MR/Blueprints/BP_Room.BP_Room_C"))
      (`/Engine/EditorBlueprintResources/StandardMacros.IsValid` _returnvalue
        (:`Is Valid`
          (set `self.RoomRef` _returnvalue))))))

(event `PrisonDropped`
  (bind _returnvalue (`GameplayStatics.GetActorOfClass` "/Game/PLK_MR/Blueprints/Widget/BP_ResultMenu.BP_ResultMenu_C"))
  (`/Game/PLK_MR/Blueprints/Widget/BP_ResultMenu.GameEnd` _returnvalue true (`self.TotalKillCount`) (`/Game/PLK_MR/Blueprints/BP_VRPawn.Hp` (`/Game/PLK_MR/Library/BP_FunctionLibrary.Get VR Pawn`)) (`self.TimeSpent`) "NewEnumerator5")
  (`GameplayStatics.PlaySound2D` "/Game/PLK_MR/Blueprints/Sound/PrisonFall.PrisonFall" 1.0 1.0 0.0 null null))

(event `self.ReceiveTick`
  (params (DeltaSeconds :type "Float (single-precision)"))
  (if (`self.GameStarted`)
    (bind _output_get (set `self.TimeSpent` (+ (`self.TimeSpent`) DeltaSeconds)))
    (if (> _output_get 600.0)
      (`self.Losing`))))

(event `CompleteLevels`
  ;[1 1 1] Complete Levels
  (`/Game/PLK_MR/Blueprints/BP_Room.StopSpawning` (`self.RoomRef`))
  (`self.DeleteAllEnemy`)
  (`/Game/PLK_MR/GameModes/SharedSpaces/GS_PLK.GS_ShowNewQuestionAnswer` (cast `/Game/PLK_MR/GameModes/SharedSpaces/GS_PLK` (`GameplayStatics.GetGameState`) :!pure true)))

(event `Levels_Changing`
  (params (Levels :type "/Game/PLK_MR/Blueprints/Enum/Enum_GameLevels Enum" :default "NewEnumerator6"))
  ;[1 1 1] Levels Changing
  (bind _levels (`/Game/PLK_MR/Library/BP_FunctionLibrary.SetGameLevels` Levels))
  (`self.RoomRef`
    (:`then`
      _)
    (:`else`
      (bind _returnvalue (`GameplayStatics.GetActorOfClass` "/Game/PLK_MR/Blueprints/BP_Room.BP_Room_C"))
      (set `self.RoomRef` _returnvalue)))
  (switch `/Game/PLK_MR/Blueprints/Enum/Enum_GameLevels` _levels
    (:`NewEnumerator1`
      (`/Game/PLK_MR/Blueprints/BP_Room.StartSpawningEnemies` (`self.RoomRef`) _levels :!label _label))
    (:`NewEnumerator2`
      (goto _label))
    (:`NewEnumerator3`
      (goto _label))
    (:`NewEnumerator5`
      (`/Game/PLK_MR/Blueprints/BP_Room.SpawnBoss` (`self.RoomRef`))
      (`/Game/PLK_MR/Blueprints/Components/BP_BGMController.ChangeMusic` (`/Game/PLK_MR/Blueprints/BP_VRPawn.BP_BGMController` (`/Game/PLK_MR/Library/BP_FunctionLibrary.Get VR Pawn`)) "NewEnumerator3"))))

(event `Next Levels`
  ;[1 1 1] Complete Levels
  (`self.Levels_Changing` (cast `/Game/PLK_MR/Blueprints/Enum/Enum_GameLevels` (+ (`self.Level`) 1))))

(event `SpawnNewWeapon`
  (params (Gun :type "/Game/PLK_MR/Blueprints/Enum/Enum_GunType Enum" :default "NewEnumerator5"))
  ;[1 1 1] Spawn New Weapon
  (bind _outactors (`GameplayStatics.GetAllActorsOfClass` "/Game/PLK_MR/Blueprints/Gun/BP_Gun.BP_Gun_C"))
  (for _array_element _outactors
    (if (`|EnumInequality` Gun (`/Game/PLK_MR/Blueprints/Gun/BP_Gun.GunType` _array_element))
      (`|SpawnActorFromClass` (select `/Game/PLK_MR/Blueprints/Enum/Enum_GunType` Gun :`NewEnumerator0` "/Game/PLK_MR/Blueprints/Gun/BP_Handgun.BP_Handgun_C" :`NewEnumerator1` "/Game/PLK_MR/Blueprints/Gun/BP_Shotgun.BP_Shotgun_C" :`NewEnumerator2` "/Game/PLK_MR/Blueprints/Gun/BP_Sniper.BP_Sniper_C" :`NewEnumerator3` "/Game/PLK_MR/Blueprints/Gun/BP_MachineGun.BP_MachineGun_C" :`NewEnumerator4` "/Game/PLK_MR/Blueprints/Gun/BP_Laser.BP_Laser_C" :!type "Actor Class Reference") (`KismetMathLibrary.MakeTransform` (`self.K2_GetActorLocation` _array_element)) "AlwaysSpawn" "MultiplyWithRoot" null null)
      (`/Game/PLK_MR/Blueprints/Gun/BP_Gun.Destroy` _array_element)
      (break))))

(event `StartGame`
  (bind _playerpawn (`/Game/PLK_MR/Library/BP_FunctionLibrary.Get VR Pawn`))
  ;[1 1 1] Start Game
  (`|ExecutionSequence`
    (:`then_0`
      (`self.Reset All`)
      (`self.Levels_Changing` "NewEnumerator1")
      (set `self.TimeSpent` 0.0)
      (set `self.GameStarted` true)
      (`/Game/PLK_MR/GameModes/SharedSpaces/GS_PLK.GS_NewGameStart` (cast `/Game/PLK_MR/GameModes/SharedSpaces/GS_PLK` (`GameplayStatics.GetGameState`) :!pure true))
      (`/Game/PLK_MR/Blueprints/Components/BP_BGMController.ChangeMusic` (`/Game/PLK_MR/Blueprints/BP_VRPawn.BP_BGMController` (`/Game/PLK_MR/Library/BP_FunctionLibrary.Get VR Pawn`)) "NewEnumerator2"))
    (:`then_1`
      (`|SpawnActorFromClass` "/Game/PLK_MR/Blueprints/Gun/BP_Handgun.BP_Handgun_C" (`KismetMathLibrary.MakeTransform` (`SceneComponent.K2_GetComponentLocation` (`/Game/PLK_MR/Blueprints/BP_VRPawn.MotionControllerL` _playerpawn))) "AlwaysSpawn" "MultiplyWithRoot" null "NewEnumerator0" null))
    (:`then_2`
      (`|SpawnActorFromClass` "/Game/PLK_MR/Blueprints/Gun/BP_Handgun.BP_Handgun_C" (`KismetMathLibrary.MakeTransform` (`SceneComponent.K2_GetComponentLocation` (`/Game/PLK_MR/Blueprints/BP_VRPawn.MotionControllerR` _playerpawn))) "AlwaysSpawn" "MultiplyWithRoot" null "NewEnumerator0" null))))

(event `AnswerBossQuestion`
  (params (`bCorrect?` :type Boolean))
  (bind _timespent (`self.TimeSpent`))
  ;[1 1 1] Answer Boss Question
  (bind _bossref (`self.BossRef`)
    (:`then`
      (if `bCorrect?`
        (`/Game/PLK_MR/Blueprints/BP_Room.StopSpawning` (`self.RoomRef`))
        (`GameplayStatics.PlaySound2D` "/Game/PLK_MR/Blueprints/Sound/Correct.Correct" 1.0 1.0 0.0 null null)
        (bind _output_get (set `/Game/PLK_MR/Blueprints/BP_Boss.Hp` (- (`/Game/PLK_MR/Blueprints/BP_Boss.Hp` _bossref) 1) _bossref))
        (`/Game/PLK_MR/Blueprints/Widget/WBP_BossHp.SetHpBar` (cast `/Game/PLK_MR/Blueprints/Widget/WBP_BossHp` (`WidgetComponent.GetWidget` (`/Game/PLK_MR/Blueprints/BP_Boss.Hp_Widget` (`self.BossRef`))) :!pure true) _output_get)
        (if (<= _output_get 0)
          (`self.K2_DestroyActor` (`self.BossRef`))
          (`|ExecutionSequence`
            (:`then_0`
              (set `self.GameStarted` false)
              (bind _returnvalue (`GameplayStatics.GetActorOfClass` "/Game/PLK_MR/Blueprints/Widget/BP_ResultMenu.BP_ResultMenu_C"))
              (`/Game/PLK_MR/Blueprints/Widget/BP_ResultMenu.GameEnd` _returnvalue false (`self.TotalKillCount`) (`/Game/PLK_MR/Blueprints/BP_VRPawn.Hp` (`/Game/PLK_MR/Library/BP_FunctionLibrary.Get VR Pawn`)) _timespent (select `bool` (<= _timespent 420.0) :`false` (select `bool` (<= _timespent 480.0) :`false` (select `bool` (<= _timespent 540.0) :`false` "NewEnumerator4" :`true` "NewEnumerator3" :!type "/Game/PLK_MR/Blueprints/Enum/Enum_Grade Enum") :`true` "NewEnumerator2") :`true` "NewEnumerator1"))
              (`/Game/PLK_MR/Blueprints/Components/BP_BGMController.ChangeMusic` (`/Game/PLK_MR/Blueprints/BP_VRPawn.BP_BGMController` (`/Game/PLK_MR/Library/BP_FunctionLibrary.Get VR Pawn`)) "NewEnumerator4")
              (`GameplayStatics.PlaySound2D` "/Game/PLK_MR/Blueprints/Sound/SoundEffect/bigbossdie.bigbossdie" 1.0 1.0 0.0 null null))
            (:`then_1`
              (bind _outactors (`GameplayStatics.GetAllActorsOfClass` "/Game/PLK_MR/Blueprints/Gun/BP_Gun.BP_Gun_C"))
              (for _array_element _outactors
                (`/Game/PLK_MR/Blueprints/Gun/BP_Gun.Destroy` _array_element))
              (bind _outactors_2 (`GameplayStatics.GetAllActorsOfClass` "/Game/PLK_MR/Blueprints/BP_Chest.BP_Chest_C"))
              (for _array_element_2 _outactors_2
                (`self.K2_DestroyActor` _array_element_2))))
          (else
            (`KismetSystemLibrary.Delay` 2.0)
            (`/Game/PLK_MR/Blueprints/BP_Room.StartSpawningEnemies` (`self.RoomRef`) "NewEnumerator5")))
        (else
          (`GameplayStatics.PlaySound2D` "/Game/PLK_MR/Blueprints/Sound/Wrong.Wrong" 1.0 1.0 0.0 null null)
          (`/Game/PLK_MR/Blueprints/BP_Boss.Attack` _bossref))))
    (:`else`)))

(event `Reset All`
  ;[1 1 1] Reset All
  (`|ExecutionSequence`
    (:`then_0`
      (set `self.Level` "NewEnumerator0")
      (bind _outactors (`GameplayStatics.GetAllActorsOfClass` "/Game/PLK_MR/Blueprints/Gun/BP_Gun.BP_Gun_C"))
      (for _array_element _outactors
        (`/Game/PLK_MR/Blueprints/Gun/BP_Gun.Destroy` _array_element))
      (bind _outactors_2 (`GameplayStatics.GetAllActorsOfClass` "/Game/PLK_MR/Blueprints/BP_Chest.BP_Chest_C"))
      (for _array_element_2 _outactors_2
        (`self.K2_DestroyActor` _array_element_2)))
    (:`then_1`
      (`self.Update_PlayerCoins` 998)
      (bind _output_get (set `self.TempKillCount` 0))
      (`/Game/PLK_MR/GameModes/SharedSpaces/GS_PLK.GS_KillAmountUpdate` (cast `/Game/PLK_MR/GameModes/SharedSpaces/GS_PLK` (`GameplayStatics.GetGameState`) :!pure true) _output_get)
      (bind _output_get_2 (set `/Game/PLK_MR/Blueprints/BP_VRPawn.Hp` 100 (`/Game/PLK_MR/Library/BP_FunctionLibrary.Get VR Pawn`)))
      (`/Game/PLK_MR/GameModes/SharedSpaces/GS_PLK.GS_HpUpdate` (cast `/Game/PLK_MR/GameModes/SharedSpaces/GS_PLK` (`GameplayStatics.GetGameState`) :!pure true) _output_get_2))
    (:`then_2`
      (set `self.TotalKillCount` 0))))

(event `Update_PlayerCoins`
  (params (int :type Integer))
  (bind _asgs_plk (cast `/Game/PLK_MR/GameModes/SharedSpaces/GS_PLK` (`GameplayStatics.GetGameState`) :!pure true))
  ;[1 1 1] Player Info Update
  (if (== int 999)
    (bind _output_get (set `self.Coins` 0))
    (`/Game/PLK_MR/GameModes/SharedSpaces/GS_PLK.GS_CoinsUpdate` _asgs_plk _output_get)
    (else
      (bind _output_get_2 (set `self.Coins` (+ (`self.Coins`) int)))
      (`/Game/PLK_MR/GameModes/SharedSpaces/GS_PLK.GS_CoinsUpdate` _asgs_plk _output_get_2))))

(event `GetItem`
  (params (Items :type "/Game/PLK_MR/Blueprints/Enum/Enum_Item Enum" :default "NewEnumerator0"))
  ;[1 1 1] Get Item
  (switch `/Game/PLK_MR/Blueprints/Enum/Enum_Item` Items
    (:`NewEnumerator1`
      (bind _asbp_vrpawn (cast `/Game/PLK_MR/Blueprints/BP_VRPawn` (`self.GetPawn`)))
      (`/Game/PLK_MR/Blueprints/BP_VRPawn.DamagePlayer` _asbp_vrpawn -20))
    (:`NewEnumerator2`
      (`self.Update_PlayerCoins` 20))
    (:`NewEnumerator3`
      (`KismetSystemLibrary.PrintString` "Pain decrease"))))

(event `Update_PlayerKills`
  (params (Int :type Integer))
  ;[1 1 1] Player Info Update
  (`|ExecutionSequence`
    (:`then_0`
      (bind _output_get (set `self.TempKillCount` (+ (`self.TempKillCount`) Int)))
      (`/Game/PLK_MR/GameModes/SharedSpaces/GS_PLK.GS_KillAmountUpdate` (cast `/Game/PLK_MR/GameModes/SharedSpaces/GS_PLK` (`GameplayStatics.GetGameState`) :!pure true) _output_get)
      (if (>= (`self.TempKillCount`) (`BlueprintMapLibrary.Map_Find` (`self.LevelsClearScore`) (`self.Level`)))
        (switch `/Game/PLK_MR/Blueprints/Enum/Enum_GameLevels` (`self.Level`)
          (:`NewEnumerator1`
            (`self.CompleteLevels` :!label _label_2)
            (set `self.TempKillCount` 0))
          (:`NewEnumerator2`
            (goto _label_2))
          (:`NewEnumerator3`
            (goto _label_2))
          (:`NewEnumerator5`
            (`/Game/PLK_MR/Blueprints/BP_Boss.ShowWeakpoint` (`self.BossRef`))
            (`/Game/PLK_MR/Blueprints/BP_Room.StopSpawning` (`self.RoomRef`))
            (set `self.TempKillCount` 0)
            (`self.DeleteAllEnemy`)))))
    (:`then_1`
      (set `self.TotalKillCount` (+ (`self.TotalKillCount`) Int)))))

(event `ChangeGodMode`
  (bind _output_get (set `self.GodMode` (not (`self.GodMode`))))
  (`/Game/PLK_MR/GameModes/SharedSpaces/GS_PLK.GS_GodModeUpdate` (cast `/Game/PLK_MR/GameModes/SharedSpaces/GS_PLK` (`GameplayStatics.GetGameState`) :!pure true) _output_get))

(fn `DeleteAllEnemy`
  (bind _outactors (`GameplayStatics.GetAllActorsOfClass` "/Game/PLK_MR/Blueprints/Enemy/BP_BaseEnemy.BP_BaseEnemy_C"))
  (for _array_element _outactors
    (`/Game/PLK_MR/Blueprints/Enemy/BP_BaseEnemy.DestroySelf` _array_element))
  (bind _outactors_2 (`GameplayStatics.GetAllActorsOfClass` "/Game/PLK_MR/Blueprints/BP_Portal.BP_Portal_C"))
  (for _array_element_2 _outactors_2
    (`self.K2_DestroyActor` _array_element_2)))

(fn `HpDecreased`
  (params (Int :type Integer))
  (set `self.HpDecrease` (+ (`self.HpDecrease`) Int)))

(fn `UserConstructionScript`)