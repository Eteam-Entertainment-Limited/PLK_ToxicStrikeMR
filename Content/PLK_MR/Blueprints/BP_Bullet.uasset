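; BP_Bullet is a VR projectile that damages enemies and hits boss weak points.
; It launches forward by a speed-scaled impulse on its sphere collision, and a looping timer destroys it beyond a horizontal distance from the VR pawn's camera.
; Overlapping a BP_BaseEnemy applies damage, spawns a burst actor matching the gun type and destroys the bullet.
; On BP_Boss, component tags select which weak point to hit, and only tagged hits destroy it.
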(event `self.ReceiveBeginPlay`
  ;[1 1 1] Begin play
  (`PrimitiveComponent.AddImpulse` (`self.SphereCollision`) (* (`self.GetActorForwardVector`) 1000.0 (`self.Speed`)) "None" true)
  (`KismetSystemLibrary.K2_SetTimerDelegate` (delegate `CheckDistance`) 0.1 true)
  (`ActorComponent.Deactivate` (`self.Burst`)))

(event `CheckDistance`
  ;[1 1 1] Begin play
  (if (not (`self.DistanceDetecter` 1000.0))
    (`self.K2_DestroyActor`)))

(event `self.SphereCollision.OnComponentBeginOverlap`
  (params (OverlappedComponent :type "PrimitiveComponent Object Reference") (OtherActor :type "Actor Object Reference") (OtherComp :type "PrimitiveComponent Object Reference") (OtherBodyIndex :type Integer) (bFromSweep :type Boolean) (SweepResult :type "HitResult Structure (by ref)"))
  ;[1 1 1] Bullet hit
  (`|ExecutionSequence`
    (:`then_0`
      (bind _asbp_base_enemy (cast `/Game/PLK_MR/Blueprints/Enemy/BP_BaseEnemy` OtherActor))
      (`/Game/PLK_MR/Blueprints/Enemy/BP_BaseEnemy.Damaged` _asbp_base_enemy (`self.Atk`) false)
      (`|SpawnActorFromClass` "/Game/PLK_MR/Blueprints/BP_BulletBurst.BP_BulletBurst_C" (`KismetMathLibrary.MakeTransform` (`SceneComponent.K2_GetComponentLocation` (`self.SphereCollision`))) "Undefined" "MultiplyWithRoot" null (`self.GunType`) null)
      (`self.K2_DestroyActor`))
    (:`then_1`
      (bind _asbp_boss (cast `/Game/PLK_MR/Blueprints/BP_Boss` OtherActor))
      (if (`ActorComponent.ComponentHasTag` OtherComp "Ans1")
        (`/Game/PLK_MR/Blueprints/BP_Boss.HitWeakpoint` _asbp_boss 1)
        (`self.K2_DestroyActor` :!label _label)
        (elif (`ActorComponent.ComponentHasTag` OtherComp "Ans2")
          (`/Game/PLK_MR/Blueprints/BP_Boss.HitWeakpoint` _asbp_boss 2)
          (goto _label)
          (elif (`ActorComponent.ComponentHasTag` OtherComp "Ans3")
            (`/Game/PLK_MR/Blueprints/BP_Boss.HitWeakpoint` _asbp_boss 3)
            (goto _label)))))))

(fn `DistanceDetecter`
  (params (Distance :type "Float (double-precision)"))
  (returns (`PlayerInDistance?` :type Boolean) (ActualDistance :type "Float (double-precision)"))
  (bind (_returnvalue_x _returnvalue_y) (`KismetMathLibrary.BreakVector` (`self.K2_GetActorLocation`)))
  (bind (_returnvalue_x_2 _returnvalue_y_2) (`KismetMathLibrary.BreakVector` (`SceneComponent.K2_GetComponentLocation` (`/Game/PLK_MR/Blueprints/BP_VRPawn.Camera` (`/Game/PLK_MR/Library/BP_FunctionLibrary.Get VR Pawn`)))))
  (bind _returnvalue (`KismetMathLibrary.Vector_Distance` (`KismetMathLibrary.MakeVector` _returnvalue_x _returnvalue_y) (`KismetMathLibrary.MakeVector` _returnvalue_x_2 _returnvalue_y_2)))
  (return (<= _returnvalue Distance) _returnvalue))

(fn `UserConstructionScript`)