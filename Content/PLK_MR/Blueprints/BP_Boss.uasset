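; VR quiz boss that exposes three answer weak points for questions from DT_BossQuestion, and attacks with a shockwave that damages the player and starts enemy spawning.
; ShowWeakpoint reveals the question and colliders after a sound-timed delay, while Tick turns answers toward the camera.
; Hits fill per-answer progress circles; a full circle reports right or wrong to the player state and resets.
; Questions are shuffled, and correctly answered ones are removed.
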(event `self.ReceiveBeginPlay`
  (bind _q_text (`self.Q_Text`))
  ;[1 1 1] Begin play
  (`|ExecutionSequence`
    (:`then_0`
      (`self.PlayerPawn`
        (:`then`)
        (:`else`
          (bind _asbp_vrpawn (cast `/Game/PLK_MR/Blueprints/BP_VRPawn` (`GameplayStatics.GetPlayerPawn` 0)))
          (set `self.PlayerPawn` _asbp_vrpawn))))
    (:`then_1`
      (`PrimitiveComponent.SetCollisionEnabled` (`self.Ans3_Model`) "NoCollision")
      (`PrimitiveComponent.SetCollisionEnabled` (`self.Ans2_Model`) "NoCollision")
      (`PrimitiveComponent.SetCollisionEnabled` (`self.Ans1_Model`) "NoCollision"))
    (:`then_2`
      (`/Game/PLK_MR/Blueprints/Widget/WBP_BossQuestion.SetText` (cast `/Game/PLK_MR/Blueprints/Widget/WBP_BossQuestion` (`WidgetComponent.GetWidget` _q_text) :!pure true) "" "" "" "")
      (`SceneComponent.SetHiddenInGame` _q_text true false))
    (:`then_3`
      (`self.Reset States`))
    (:`then_4`
      (set `self.Hp` 5)
      (bind _outrownames (`DataTableFunctionLibrary.GetDataTableRowNames` "/Game/PLK_MR/Table/DT_BossQuestion.DT_BossQuestion"))
      (bind _output_get (set `self.Questions` _outrownames))
      (`KismetArrayLibrary.Array_Shuffle` _output_get))
    (:`then_5`
      (`/Game/PLK_MR/Blueprints/Widget/WBP_CircleProgressbar.SetAnswer` (cast `/Game/PLK_MR/Blueprints/Widget/WBP_CircleProgressbar` (`WidgetComponent.GetWidget` (`self.Ans1_Widget`)) :!pure true) "A")
      (`/Game/PLK_MR/Blueprints/Widget/WBP_CircleProgressbar.SetAnswer` (cast `/Game/PLK_MR/Blueprints/Widget/WBP_CircleProgressbar` (`WidgetComponent.GetWidget` (`self.Ans2_Widget`)) :!pure true) "B")
      (`/Game/PLK_MR/Blueprints/Widget/WBP_CircleProgressbar.SetAnswer` (cast `/Game/PLK_MR/Blueprints/Widget/WBP_CircleProgressbar` (`WidgetComponent.GetWidget` (`self.Ans3_Widget`)) :!pure true) "C")
      (`ActorComponent.Deactivate` (`self.NS_Shockwave`)))))

(event `self.ReceiveTick`
  (params (DeltaSeconds :type "Float (single-precision)"))
  ;[1 1 1] Event Tick
  (`|ExecutionSequence`
    (:`then_0`
      (`SceneComponent.K2_SetWorldRotation` (`self.Ans1`) (`KismetMathLibrary.FindLookAtRotation` (`SceneComponent.K2_GetComponentLocation` (`self.Ans1`)) (`SceneComponent.K2_GetComponentLocation` (`/Game/PLK_MR/Blueprints/BP_VRPawn.Camera` (`self.PlayerPawn`)))) false false))
    (:`then_1`
      (`SceneComponent.K2_SetWorldRotation` (`self.Ans2`) (`KismetMathLibrary.FindLookAtRotation` (`SceneComponent.K2_GetComponentLocation` (`self.Ans2`)) (`SceneComponent.K2_GetComponentLocation` (`/Game/PLK_MR/Blueprints/BP_VRPawn.Camera` (`self.PlayerPawn`)))) false false))
    (:`then_2`
      (`SceneComponent.K2_SetWorldRotation` (`self.Ans3`) (`KismetMathLibrary.FindLookAtRotation` (`SceneComponent.K2_GetComponentLocation` (`self.Ans3`)) (`SceneComponent.K2_GetComponentLocation` (`/Game/PLK_MR/Blueprints/BP_VRPawn.Camera` (`self.PlayerPawn`)))) false false))))

(event `ShowWeakpoint`
  ;[1 1 1] ShowWeakPoint
  (`GameplayStatics.PlaySound2D` "/Game/PLK_MR/Blueprints/Sound/SoundEffect/BigBoss.BigBoss" 1.0 1.0 0.0 null null)
  (set `self.ShowWeak` true)
  (`KismetSystemLibrary.Delay` 3.71)
  (`self.WeakPointAppear`))

(event `WeakPointAppear`
  (bind _q_text (`self.Q_Text`))
  ;[1 1 1] ShowWeakPoint
  (`SceneComponent.SetHiddenInGame` (`self.Ans1_Widget`) false false)
  (`SceneComponent.SetHiddenInGame` (`self.Ans2_Widget`) false false)
  (`SceneComponent.SetHiddenInGame` (`self.Ans3_Widget`) false false)
  (`PrimitiveComponent.SetCollisionEnabled` (`self.Ans3_Model`) "QueryAndPhysics")
  (`PrimitiveComponent.SetCollisionEnabled` (`self.Ans2_Model`) "QueryAndPhysics")
  (`PrimitiveComponent.SetCollisionEnabled` (`self.Ans1_Model`) "QueryAndPhysics")
  (bind _returnvalue (`|GetDataTableRow` "/Game/PLK_MR/Table/DT_BossQuestion.DT_BossQuestion" (`|GetArrayItem` (`self.Questions`)))
    (:`then`
      (bind (_question _a _b _c _correctans) (break `/Game/PLK_MR/Table/Stru_BossQuestion` _returnvalue))
      (`/Game/PLK_MR/Blueprints/Widget/WBP_BossQuestion.SetText` (cast `/Game/PLK_MR/Blueprints/Widget/WBP_BossQuestion` (`WidgetComponent.GetWidget` _q_text) :!pure true) _question _a _b _c)
      (`SceneComponent.SetHiddenInGame` _q_text false false)
      (set `self.CorrectAns` _correctans))))

(event `HitWeakpoint`
  (params (AnsNum :type Integer))
  ;[1 1 1] Weak Point Hit
  (switch `int` AnsNum
    (:`1`
      (set `self.A_Percent` (+ (`self.A_Percent`) 10.0)))
    (:`2`
      (set `self.B_Percent` (+ (`self.B_Percent`) 10.0)))
    (:`3`
      (set `self.C_Percent` (+ (`self.C_Percent`) 10.0))))
  (`/Game/PLK_MR/Blueprints/Widget/WBP_CircleProgressbar.Set Percent` (cast `/Game/PLK_MR/Blueprints/Widget/WBP_CircleProgressbar` (`WidgetComponent.GetWidget` (select `int` AnsNum :`0` null :`1` (`self.Ans1_Widget`) :`2` (`self.Ans2_Widget`) :`3` (`self.Ans3_Widget`))) :!pure true) (select `int` AnsNum :`0` 0.0 :`1` (`self.A_Percent`) :`2` (`self.B_Percent`) :`3` (`self.C_Percent`)))
  (`self.CheckAnswered` AnsNum))

(event `Attack`
  (bind _playerpawn (`/Game/PLK_MR/Library/BP_FunctionLibrary.Get VR Pawn`))
  ;[1 1 1] Attack
  (`GameplayStatics.PlaySound2D` "/Game/PLK_MR/Blueprints/Sound/BossAtk.BossAtk" 1.0 1.0 0.0 null null)
  (`KismetSystemLibrary.Delay` 5.58)
  (`ActorComponent.Activate` (`self.NS_Shockwave`) true)
  (`/Game/PLK_MR/Blueprints/BP_VRPawn.CameraShake` _playerpawn)
  (`/Game/PLK_MR/Blueprints/BP_VRPawn.DamagePlayer` _playerpawn 20)
  (`KismetSystemLibrary.Delay` 2.0)
  (`/Game/PLK_MR/Blueprints/BP_Room.StartSpawningEnemies` (`/Game/PLK_MR/GameModes/SharedSpaces/BP_PLKPlayerState.RoomRef` (`/Game/PLK_MR/Library/BP_FunctionLibrary.GetOwningPlayerState`)) "NewEnumerator5"))

(event `CheckAnswered`
  (params (AnsNum :type Integer))
  (bind _questions (`self.Questions`))
  (bind _returnvalue (== (`self.CorrectAns`) AnsNum))
  ;[1 1 1] Check Answer
  (if (>= (select `int` AnsNum :`0` 0.0 :`1` (`self.A_Percent`) :`2` (`self.B_Percent`) :`3` (`self.C_Percent`)) 100.0)
    (`|ExecutionSequence`
      (:`then_0`
        (if _returnvalue
          (`KismetArrayLibrary.Array_RemoveItem` _questions (`|GetArrayItem` _questions))
          (`KismetArrayLibrary.Array_Shuffle` (`self.Questions`))
          (set `self.bIsCorrect` true)
          (`GameplayStatics.PlaySound2D` "/Game/PLK_MR/Blueprints/Sound/SoundEffect/bigbossdie.bigbossdie" 1.0 1.0 0.0 null null)
          (else
            (set `self.bIsCorrect` false))))
      (:`then_1`
        (`/Game/PLK_MR/GameModes/SharedSpaces/BP_PLKPlayerState.AnswerBossQuestion` (`/Game/PLK_MR/Library/BP_FunctionLibrary.GetOwningPlayerState`) _returnvalue)
        (`self.Reset States`)
        (set `self.ShowWeak` false)
        (set `self.WeakPointHitted` true)
        (`KismetSystemLibrary.Delay` 0.5)
        (set `self.WeakPointHitted` false)))))

(event `Reset States`
  ;[1 1 1] Reset
  (`|ExecutionSequence`
    (:`then_0`
      (set `self.A_Percent` 0.0)
      (set `self.B_Percent` 0.0)
      (set `self.C_Percent` 0.0)
      (`/Game/PLK_MR/Blueprints/Widget/WBP_CircleProgressbar.Set Percent` (cast `/Game/PLK_MR/Blueprints/Widget/WBP_CircleProgressbar` (`WidgetComponent.GetWidget` (`self.Ans1_Widget`)) :!pure true) 0.0)
      (`/Game/PLK_MR/Blueprints/Widget/WBP_CircleProgressbar.Set Percent` (cast `/Game/PLK_MR/Blueprints/Widget/WBP_CircleProgressbar` (`WidgetComponent.GetWidget` (`self.Ans2_Widget`)) :!pure true) 0.0)
      (`/Game/PLK_MR/Blueprints/Widget/WBP_CircleProgressbar.Set Percent` (cast `/Game/PLK_MR/Blueprints/Widget/WBP_CircleProgressbar` (`WidgetComponent.GetWidget` (`self.Ans3_Widget`)) :!pure true) 0.0)
      (`SceneComponent.SetHiddenInGame` (`self.Q_Text`) true false)
      (`SceneComponent.SetHiddenInGame` (`self.Ans1_Widget`) true false)
      (`SceneComponent.SetHiddenInGame` (`self.Ans2_Widget`) true false)
      (`SceneComponent.SetHiddenInGame` (`self.Ans3_Widget`) true false))
    (:`then_1`
      (`PrimitiveComponent.SetCollisionEnabled` (`self.Ans3_Model`) "NoCollision")
      (`PrimitiveComponent.SetCollisionEnabled` (`self.Ans1_Model`) "NoCollision")
      (`PrimitiveComponent.SetCollisionEnabled` (`self.Ans2_Model`) "NoCollision"))))

(fn `UserConstructionScript`)