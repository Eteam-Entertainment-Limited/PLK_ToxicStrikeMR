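; BP_Prison is a prison actor whose mesh drops into place as soon as it spawns.
; A timeline lowers the static mesh along Z from a raised offset.
; When the drop finishes, it shakes the VR pawn's camera, waits briefly, then notifies the owning player state through PrisonDropped.
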(event `self.ReceiveBeginPlay`
  (`self.Drop`))

(event `Drop`
  (bind _staticmesh (`self.StaticMesh`))
  (bind (_relativelocation_x _relativelocation_y) (`KismetMathLibrary.BreakVector` (`SceneComponent.RelativeLocation` _staticmesh)))
  (bind (_direction _drop) (`Timeline|Dropping` :!via `PlayFromStart`)
    (:`Update`
      (`SceneComponent.K2_SetRelativeLocation` _staticmesh (`KismetMathLibrary.MakeVector` _relativelocation_x _relativelocation_y (`KismetMathLibrary.MapRangeClamped` _drop 0.0 1.0 200.0 100.0)) false true))
    (:`Finished`
      (`/Game/PLK_MR/Blueprints/BP_VRPawn.CameraShake` (`/Game/PLK_MR/Library/BP_FunctionLibrary.Get VR Pawn`))
      (`KismetSystemLibrary.Delay` 1.0)
      (`/Game/PLK_MR/GameModes/SharedSpaces/BP_PLKPlayerState.PrisonDropped` (`/Game/PLK_MR/Library/BP_FunctionLibrary.GetOwningPlayerState`)))))

(fn `UserConstructionScript`)