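; BP_Cube is a cube actor that can be highlighted on hover and launched upward on command.
; On BeginPlay it creates a dynamic instance of M_Cube and stores it.
; SetHovered switches that instance's Emissive parameter between the hover and default colors.
; ExplodeCube, despite its name, only applies a strong physics impulse in a random direction within a cone around up.
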(event `self.ReceiveBeginPlay`
  (bind _returnvalue (`PrimitiveComponent.CreateDynamicMaterialInstance` (`self.Cube`) 0 "/Game/PLK_MR/Materials/M_Cube.M_Cube" "None"))
  (set `self.MaterialInstance` _returnvalue))

(event `Set Hovered`
  (params (IsHovered :type Boolean))
  (`MaterialInstanceDynamic.SetVectorParameterValue` (`self.MaterialInstance`) "Emissive" (select `bool` IsHovered :`false` (`self.DefaultColor`) :`true` (`self.HoverColor`))))

(event `Explode Cube`
  (`PrimitiveComponent.AddImpulse` (`self.Cube`) (* (`KismetMathLibrary.RandomUnitVectorInConeInDegrees` (`KismetMathLibrary.Vector_Up`) 30.0) 10000.0) "None" false))

(fn `UserConstructionScript`)