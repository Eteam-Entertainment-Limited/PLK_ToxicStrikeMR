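; BP_BaseEnemy is a VR enemy whose type (Lv1–Lv3) sets its stats, material, movement and coin reward.
; Lv1 homes on the player's camera and self-destructs on contact, Lv2 faces the player while moving horizontally, and Lv3 moves forward; room overlaps turn enemies around.
; A looping-timer routine fires bullets.
; Damage spawns damage numbers, throttles laser hits with DoOnce, and on death awards coins, kills and occasional chests.
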(event `self.ReceiveBeginPlay`
  (bind _enemytype (`self.EnemyType`))
  (`|ExecutionSequence`
    (:`then_0`
      (set `self.Hp` (select `/Game/PLK_MR/Blueprints/Structure/Enum_EnemyType` (`self.EnemyType`) :`NewEnumerator0` 5 :`NewEnumerator1` 10 :`NewEnumerator2` 30))
      (set `self.Atk` (select `/Game/PLK_MR/Blueprints/Structure/Enum_EnemyType` _enemytype :`NewEnumerator0` 5 :`NewEnumerator1` 10 :`NewEnumerator2` 15))
      (set `self.Speed` (select `/Game/PLK_MR/Blueprints/Structure/Enum_EnemyType` _enemytype :`NewEnumerator0` 75.0 :`NewEnumerator1` 100.0 :`NewEnumerator2` 75.0 :!type "Float (single-precision)"))
      (bind _asbp_vrpawn (cast `/Game/PLK_MR/Blueprints/BP_VRPawn` (`GameplayStatics.GetPlayerPawn` 0))
        (:`then`
          (bind _output_get (set `self.Player` _asbp_vrpawn)))
        (:`CastFailed`
          _))
      (`|ExecutionSequence`
        (:`then_0`
          (switch `/Game/PLK_MR/Blueprints/Structure/Enum_EnemyType` (`self.EnemyType`)
            (:`NewEnumerator0`
              (set `ProjectileMovementComponent.HomingTargetComponent` (`/Game/PLK_MR/Blueprints/BP_VRPawn.Camera` _output_get) (`self.ProjectileMovement`)))
            (:`NewEnumerator1`
              (`ActorComponent.K2_DestroyComponent` (`self.ProjectileMovement`) :!label _label))
            (:`NewEnumerator2`
              (`KismetSystemLibrary.K2_SetTimerDelegate` (`|CreateDelegate` :!event `StartShooting`) 2.0)
              (goto _label))))
        (:`then_1`)))
    (:`then_1`
      (`PrimitiveComponent.SetMaterial` (`self.Sphere`) 0 (select `/Game/PLK_MR/Blueprints/Structure/Enum_EnemyType` (`self.EnemyType`) :`NewEnumerator0` "/AnimationSharing/AnimSharingBlue.AnimSharingBlue" :`NewEnumerator1` "/AnimationSharing/AnimSharingGreen.AnimSharingGreen" :`NewEnumerator2` "/AnimationSharing/AnimSharingRed.AnimSharingRed" :!type "MaterialInterface Object Reference"))
      (`KismetSystemLibrary.K2_SetTimerDelegate` (delegate `Spawned`) 0.5))))

(event `Spawned`
  (set `self.JustSpawned` false))

(event `CustomEvent`
  (`self.Damaged` 5))

(event `self.ReceiveTick`
  (params (DeltaSeconds :type "Float (single-precision)"))
  (bind _returnvalue (* (`self.GetActorForwardVector`) (`self.Speed`) (`GameplayStatics.GetWorldDeltaSeconds`)))
  (`|ExecutionSequence`
    (:`then_0`
      (switch `/Game/PLK_MR/Blueprints/Structure/Enum_EnemyType` (`self.EnemyType`)
        (:`NewEnumerator0`
          _)
        (:`NewEnumerator1`
          _))
      (`self.K2_SetActorRotation` (`KismetMathLibrary.FindLookAtRotation` (`SceneComponent.K2_GetComponentLocation` (`self.SkeletalMesh`)) (`SceneComponent.K2_GetComponentLocation` (`/Game/PLK_MR/Blueprints/BP_VRPawn.Camera` (`self.Player`)))) true))
    (:`then_1`
      (if (not (`self.bAttacking`))
        (`self.K2_AddActorWorldOffset` (select `/Game/PLK_MR/Blueprints/Structure/Enum_EnemyType` (`self.EnemyType`) :`NewEnumerator5` _returnvalue :`NewEnumerator0` _returnvalue :`NewEnumerator1` (`KismetMathLibrary.MakeVector` (.x _returnvalue) (.y _returnvalue)) :`NewEnumerator2` _returnvalue))
        (if (<= (`KismetMathLibrary.Vector_Distance` (`self.K2_GetActorLocation`) (`SceneComponent.K2_GetComponentLocation` (`/Game/PLK_MR/Blueprints/BP_VRPawn.Camera` (`self.Player`)))) 50.0)
          _)))))

(event `StartShooting`
  (bind _returnvalue (`KismetSystemLibrary.K2_SetTimer` null "Shooting" 5.0 true))
  (set `self.Shooting Timer` _returnvalue))

(event `Damaged`
  (params (Damage :type Integer) (bIsLaser :type Boolean))
  (bind _playerstate (`/Game/PLK_MR/Library/BP_FunctionLibrary.GetOwningPlayerState`))
  (if bIsLaser
    (`/Engine/EditorBlueprintResources/StandardMacros.DoOnce` false :!label _label_2
      (:`Completed`
        (`|ExecutionSequence`
          (:`then_0`
            _)
          (:`then_1`
            (`KismetSystemLibrary.Delay` 0.5)
            (goto _label_2 :!via `Reset`))))))
  (bind _output_get (set `self.Hp` (- (`self.Hp`) Damage)))
  (`|ExecutionSequence`
    (:`then_0`
      (if (<= _output_get 0)
        (`|ExecutionSequence`
          (:`then_0`
            (`/Game/PLK_MR/GameModes/SharedSpaces/BP_PLKPlayerState.Update_PlayerCoins` _playerstate (select `/Game/PLK_MR/Blueprints/Structure/Enum_EnemyType` (`self.EnemyType`) :`NewEnumerator0` 2 :`NewEnumerator1` 5 :`NewEnumerator2` 8))
            (`/Game/PLK_MR/GameModes/SharedSpaces/BP_PLKPlayerState.Update_PlayerKills` _playerstate 1)
            (if (== (`KismetMathLibrary.RandomIntegerInRange` 1 10) 5)
              (`|SpawnActorFromClass` "/Game/PLK_MR/Blueprints/BP_Chest.BP_Chest_C" (`KismetMathLibrary.MakeTransform` (`self.K2_GetActorLocation`) (`KismetMathLibrary.FindLookAtRotation` (`self.K2_GetActorLocation`) (`SceneComponent.K2_GetComponentLocation` (`/Game/PLK_MR/Blueprints/BP_VRPawn.Camera` (`/Game/PLK_MR/Library/BP_FunctionLibrary.Get VR Pawn`))))) "Undefined" "MultiplyWithRoot" null null)))
          (:`then_1`
            (`self.DestroySelf`)))))
    (:`then_1`
      (`|SpawnActorFromClass` "/Game/PLK_MR/Blueprints/Widget/BP_Damaged.BP_Damaged_C" (`KismetMathLibrary.MakeTransform` (`self.K2_GetActorLocation`)) "Undefined" "MultiplyWithRoot" null (`KismetStringLibrary.Conv_IntToString` Damage) null))))

(event `self.HitCollider.OnComponentBeginOverlap`
  (params (OverlappedComponent :type "PrimitiveComponent Object Reference") (OtherActor :type "Actor Object Reference") (OtherComp :type "PrimitiveComponent Object Reference") (OtherBodyIndex :type Integer) (bFromSweep :type Boolean) (SweepResult :type "HitResult Structure (by ref)"))
  (`|ExecutionSequence`
    (:`then_0`
      (if (`|EnumEquality` (`self.EnemyType`) "NewEnumerator0")
        (bind _asbp_vrpawn (cast `/Game/PLK_MR/Blueprints/BP_VRPawn` OtherActor))
        (`/Game/PLK_MR/Blueprints/BP_VRPawn.DamagePlayer` _asbp_vrpawn (`self.Atk`))
        (`|ExecutionSequence`
          (:`then_1`
            (`self.DestroySelf`)))))
    (:`then_1`
      (cast `/Game/PLK_MR/Blueprints/BP_Room` OtherActor)
      (if (not (`self.JustSpawned`))
        (`self.ReverseRotation`)))))

(event `ReverseRotation`
  (bind (_returnvalue_roll _returnvalue_pitch _returnvalue_yaw) (`KismetMathLibrary.BreakRotator` (`KismetMathLibrary.FindLookAtRotation` (`self.K2_GetActorLocation`) (* (`self.GetActorForwardVector`) -200.0))))
  (`self.K2_SetActorRotation` (`KismetMathLibrary.MakeRotator` 0.0 0.0 (+ _returnvalue_yaw (`KismetMathLibrary.RandomFloatInRange` -40.0 40.0))) true))

(event `DestroySelf`
  (`self.K2_DestroyActor`))

(fn `Shooting`
  (`|SpawnActorFromClass` "/Game/PLK_MR/Blueprints/BP_EnemyBullet.BP_EnemyBullet_C" (`KismetMathLibrary.MakeTransform` (`self.K2_GetActorLocation`)) "Undefined" "MultiplyWithRoot" null 15 null))

(fn `UserConstructionScript`)