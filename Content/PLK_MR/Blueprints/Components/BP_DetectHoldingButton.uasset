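; BP_DetectHoldingButton is a component that detects a held VR controller combo to trigger spatial anchor creation and orientation.
; HoldingAButton tracks held button names in a list and starts a three-second timer once both grips and both joysticks are held.
; Any reported release cancels the timer; on completion, SuccessOrient calls CreateAnchorSaveAndOrient on the owning BP_VRPawn's SpatialAnchorManagerAC.
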(fn `Holding a Button`
  (params (` Name` :type Name) (bHolding :type Boolean))
  (bind _holdinglist (`self.HoldingList`))
  ;[1 1 1] Detect holding button
  (if bHolding
    (`KismetArrayLibrary.Array_AddUnique` _holdinglist ` Name`)
    (if (and (`KismetArrayLibrary.Array_Contains` _holdinglist "LControllerGrip") (`KismetArrayLibrary.Array_Contains` _holdinglist "RControllerGrip") (`KismetArrayLibrary.Array_Contains` _holdinglist "LControllerJoy") (`KismetArrayLibrary.Array_Contains` _holdinglist "RControllerJoy"))
      (`KismetSystemLibrary.PrintString` "1")
      (if (not (`KismetSystemLibrary.K2_IsTimerActiveHandle` (`self.SuccessTimer`)))
        (bind _returnvalue (`KismetSystemLibrary.K2_SetTimer` null "SuccessOrient" 3.0))
        (set `self.SuccessTimer` _returnvalue)))
    (else
      (`KismetArrayLibrary.Array_RemoveItem` (`self.HoldingList`) ` Name`)
      (if (`KismetSystemLibrary.K2_IsTimerActiveHandle` (`self.SuccessTimer`))
        (`KismetSystemLibrary.K2_ClearAndInvalidateTimerHandle` (`self.SuccessTimer`))
        (`KismetSystemLibrary.PrintString` "8")))))

(fn `SuccessOrient`
  (bind _asbp_vrpawn (cast `/Game/PLK_MR/Blueprints/BP_VRPawn` (`self.GetOwner`)))
  (`/Game/PLK_MR/Blueprints/Components/BP_SpatialAnchorManagerComponent.CreateAnchorSaveAndOrient` (`/Game/PLK_MR/Blueprints/BP_VRPawn.SpatialAnchorManager_AC` _asbp_vrpawn)))