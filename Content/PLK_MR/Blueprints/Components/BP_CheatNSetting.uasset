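; Component that detects secret input sequences to toggle god mode or open the settings on the VR pawn.
; Each input is appended to a list and restarts a one-second timer that clears the list when input pauses.
; The list is compared exactly against the cheat and setting sequences; a match flips GodMode on the owning player's state or calls OpenSetting on the owning BP_VRPawn, then clears the list.
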(event `self.ReceiveBeginPlay`)

(event `self.ReceiveTick`
  (params (DeltaSeconds :type "Float (single-precision)")))

(event `Input`
  (params (Input :type String))
  (bind _resettimer (`self.ResetTImer`))
  (`|ExecutionSequence`
    (:`then_0`
      (if (`KismetSystemLibrary.K2_IsTimerActiveHandle` _resettimer)
        (`KismetSystemLibrary.K2_ClearAndInvalidateTimerHandle` _resettimer))
      (bind _returnvalue (`KismetSystemLibrary.K2_SetTimer` null "Reset" 1.0))
      (set `self.ResetTImer` _returnvalue))
    (:`then_1`
      (`KismetArrayLibrary.Array_Add` (`self.InputList`) Input)
      (`self.CheckList`))))

(fn `CheckList`
  (bind _playerstate (`/Game/PLK_MR/Library/BP_FunctionLibrary.GetOwningPlayerState`))
  (if (`KismetArrayLibrary.Array_Identical` (`self.InputList`) (`self.OpenCheatList`))
    (set `/Game/PLK_MR/GameModes/SharedSpaces/BP_PLKPlayerState.GodMode` (not (`/Game/PLK_MR/GameModes/SharedSpaces/BP_PLKPlayerState.GodMode` _playerstate)) _playerstate)
    (`self.Reset`)
    (elif (`KismetArrayLibrary.Array_Identical` (`self.InputList`) (`self.OpenSettingList`))
      (bind _asbp_vrpawn (cast `/Game/PLK_MR/Blueprints/BP_VRPawn` (`self.GetOwner`)))
      (`/Game/PLK_MR/Blueprints/BP_VRPawn.OpenSetting` _asbp_vrpawn)
      (`self.Reset`))))

(fn `Reset`
  (`KismetArrayLibrary.Array_Clear` (`self.InputList`)))