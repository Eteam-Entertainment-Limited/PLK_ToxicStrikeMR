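; BP_SessionManager hosts and joins non-LAN online multiplayer sessions for the spatial anchors showcase.
; CreateSession creates a session, then opens the SA_Showcase map as a listen server on success.
; FindSessions stores the search results and automatically joins the first one, if any.
; Both events use async session nodes and report start and success or failure to Menu through StartAsync and EndAsync.
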(event `Create Session`
  (bind _menu (`self.Menu`))
  (`CreateSessionCallbackProxy.CreateSession` (`GameplayStatics.GetPlayerController` 0) 5
    (:`then`
      (`/Game/PLK_MR/Blueprints/UI/BP_Menu.Start Async` _menu))
    (:`OnSuccess`
      (`/Game/PLK_MR/Blueprints/UI/BP_Menu.End Async` _menu true)
      (`GameplayStatics.OpenLevel` "/Game/SpatialAnchorsSample/Maps/SA_Showcase" true "?listen"))
    (:`OnFailure`
      (`/Game/PLK_MR/Blueprints/UI/BP_Menu.End Async` _menu false))))

(event `Find Sessions`
  (bind _menu (`self.Menu`))
  (bind _results (`FindSessionsCallbackProxy.FindSessions` (`GameplayStatics.GetPlayerController` 0) 10)
    (:`then`
      (`/Game/PLK_MR/Blueprints/UI/BP_Menu.Start Async` _menu))
    (:`OnSuccess`
      (`/Game/PLK_MR/Blueprints/UI/BP_Menu.End Async` _menu true)
      (set `self.FoundSessions` _results)
      (if (> (`KismetArrayLibrary.Array_Length` _results) 0)
        (`JoinSessionCallbackProxy.JoinSession` (`GameplayStatics.GetPlayerController` 0) (`|GetArrayItem` (`self.FoundSessions`)))))
    (:`OnFailure`
      (`/Game/PLK_MR/Blueprints/UI/BP_Menu.End Async` _menu false))))