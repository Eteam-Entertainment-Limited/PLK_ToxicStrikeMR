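; BP_LobbyMenuManager spawns and drives the lobby main menu in the MR project.
; On BeginPlay it spawns BP_Lobby_Menu with the spatial anchor and session managers, sets it as the current menu context and registers it with SessionManager.
; Tick snaps the menu to MainMenuPositioner's transform.
; Navigation and select events forward to the current context, or directly to the main menu; an Android storage-permission request is left unconnected.
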(event `self.ReceiveBeginPlay`
  ;[1 1 1] Setting up Main Menu
  (bind _returnvalue (`|SpawnActorFromClass` "/Game/PLK_MR/Blueprints/UI/BP_Lobby_Menu.BP_Lobby_Menu_C" (`SceneComponent.K2_GetComponentToWorld` (`self.MainMenuPositioner`)) "Undefined" "OverrideRootScale" null (`self.SpatialAnchorManager`) self (`self.Session Manager`) null))
  (bind _output_get (set `self.MainMenu` _returnvalue))
  (bind _output_get_2 (set `self.CurrentMenuContext` _output_get))
  (set `/Game/PLK_MR/Blueprints/Components/BP_SessionManager.Menu` _output_get_2 (`self.Session Manager`)))

(event `self.ReceiveTick`
  (params (DeltaSeconds :type "Float (single-precision)"))
  (bind _mainmenu (`self.MainMenu`))
  ;[1 1 1] Update Main Menu position
  (`/Engine/EditorBlueprintResources/StandardMacros.IsValid` _mainmenu
    (:`Is Valid`
      (`Actor.K2_SetActorTransform` _mainmenu (`SceneComponent.K2_GetComponentToWorld` (`self.MainMenuPositioner`)) false false))))

(event `Menu Selection Up`
  ;[1 1 1] Menu Navigation
  (`/Game/PLK_MR/Blueprints/UI/BP_Menu.Menu Selection Up` (`self.CurrentMenuContext`)))

(event `Select Menu Item`
  ;[1 1 1] Running logic on selected menu item
  (`/Game/PLK_MR/Blueprints/UI/BP_Menu.Run Select` (`self.CurrentMenuContext`)))

(event `Menu Selection Down`
  ;[1 1 1] Menu Navigation
  (`/Game/PLK_MR/Blueprints/UI/BP_Menu.Menu Selection Down` (`self.CurrentMenuContext`)))

(event `Select Main Menu Item`
  (bind _mainmenu (`self.MainMenu`))
  ;[1 1 1] Running logic on selected menu item
  (`/Engine/EditorBlueprintResources/StandardMacros.IsValid` _mainmenu
    (:`Is Valid`
      (`/Game/PLK_MR/Blueprints/UI/BP_Menu.Run Select` _mainmenu))))