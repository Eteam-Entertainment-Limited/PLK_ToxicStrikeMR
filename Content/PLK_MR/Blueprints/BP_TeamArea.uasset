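; BP_TeamArea is a team zone actor that shows a red or blue area, sized by its AreaSize variable.
; On BeginPlay it scales a Cube to that size, raises it by half its height and picks the team material from IsBlue.
; The Cube's overlap event only prints a debug message when the VR pawn enters, and the construction script is empty.
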(event `self.ReceiveBeginPlay`
  (bind _cube (`self.Cube`))
  (bind (_areasize_x _areasize_y) (`KismetMathLibrary.BreakVector` (`self.AreaSize`)))
  (bind (_returnvalue_x _returnvalue_y _returnvalue_z) (`KismetMathLibrary.BreakVector` (`SceneComponent.K2_GetComponentScale` _cube)))
  (`SceneComponent.SetWorldScale3D` _cube (`KismetMathLibrary.MakeVector` (/ _areasize_x 100.0) (/ _areasize_y 100.0) _returnvalue_z))
  (`SceneComponent.K2_SetRelativeLocation` (`self.Cube`) (`KismetMathLibrary.MakeVector` 0.0 0.0 (* _returnvalue_z 50.0)) false true)
  (`PrimitiveComponent.SetMaterial` (`self.Cube`) 0 (select `bool` (`self.IsBlue?`) :`false` (`self.TeamRedMat`) :`true` (`self.TeamBlueMat`))))

(event `self.Cube.OnComponentBeginOverlap`
  (params (OverlappedComponent :type "PrimitiveComponent Object Reference") (OtherActor :type "Actor Object Reference") (OtherComp :type "PrimitiveComponent Object Reference") (OtherBodyIndex :type Integer) (bFromSweep :type Boolean) (SweepResult :type "HitResult Structure (by ref)"))
  (if (== OtherActor "/Game/PLK_MR/Blueprints/BP_VRPawn.BP_VRPawn")
    (`KismetSystemLibrary.PrintString` "Player Inside area")))

(fn `UserConstructionScript`)