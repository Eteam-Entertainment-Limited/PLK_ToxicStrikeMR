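; Base VR enemy whose type sets behavior and whose level sets stats, material and coin reward.
; Tick turns it toward the player and moves it, with Coke King bouncing off room walls.
; Space Oil, Weed and Heroin melee via delay-timed hitbox windows, while K Boy and Coke King fire timed bullet volleys.
; Damage throttles laser hits and shows damage actors; death awards coins and kills, sometimes dropping a chest.
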(event `self.ReceiveBeginPlay`
  (bind _enemylevel (`self.EnemyLevel`))
  ;[1 1 1] Begin play
  (`|ExecutionSequence`
    (:`then_0`
      (set `self.Hp` (select `/Game/PLK_MR/Blueprints/Enum/Enum_EnemyLevels` (`self.EnemyLevel`) :`NewEnumerator0` 15 :`NewEnumerator1` 30 :`NewEnumerator2` 60))
      (set `self.Atk` (select `/Game/PLK_MR/Blueprints/Enum/Enum_EnemyLevels` _enemylevel :`NewEnumerator0` 4 :`NewEnumerator1` 6 :`NewEnumerator2` 8))
      (set `self.Speed` (select `/Game/PLK_MR/Blueprints/Enum/Enum_EnemyLevels` _enemylevel :`NewEnumerator0` 75.0 :`NewEnumerator1` 100.0 :`NewEnumerator2` 100.0 :!type "Float (single-precision)"))
      (bind _asbp_vrpawn (cast `/Game/PLK_MR/Blueprints/BP_VRPawn` (`GameplayStatics.GetPlayerPawn` 0))
        (:`then`
          (bind _output_get (set `self.Player` _asbp_vrpawn)))
        (:`CastFailed`
          _))
      (`|ExecutionSequence`
        (:`then_0`
          (`ActorComponent.K2_DestroyComponent` (`self.ProjectileMovement`))
          (switch `/Game/PLK_MR/Blueprints/Enum/Enum_EnemyTypes` (`self.EnemyTypes`)
            (:`NewEnumerator3`
              (`|ExecutionSequence`
                (:`then_1`
                  (`KismetSystemLibrary.K2_SetTimerDelegate` (`|CreateDelegate` :!event `StartShooting`) 1.0 :!label _label))
                (:`then_2`
                  (`KismetSystemLibrary.Delay` 1.0)
                  (set `self.bStop` true))))
            (:`NewEnumerator4`
              (`|ExecutionSequence`
                (:`then_0`
                  (goto _label))))))))
    (:`then_1`
      (`PrimitiveComponent.SetMaterial` (`self.Sphere`) 0 (select `/Game/PLK_MR/Blueprints/Enum/Enum_EnemyLevels` (`self.EnemyLevel`) :`NewEnumerator0` "/AnimationSharing/AnimSharingBlue.AnimSharingBlue" :`NewEnumerator1` "/AnimationSharing/AnimSharingGreen.AnimSharingGreen" :`NewEnumerator2` "/AnimationSharing/AnimSharingRed.AnimSharingRed" :!type "MaterialInterface Object Reference"))
      (`KismetSystemLibrary.K2_SetTimerDelegate` (delegate `Spawned`) 0.5)
      (`GameplayStatics.PlaySoundAtLocation` (select `/Game/PLK_MR/Blueprints/Enum/Enum_EnemyTypes` (`self.EnemyTypes`) :`NewEnumerator1` "/Game/PLK_MR/Blueprints/Sound/SoundEffect/oil.oil" :`NewEnumerator2` "/Game/PLK_MR/Blueprints/Sound/SoundEffect/weed.weed" :`NewEnumerator3` "/Game/PLK_MR/Blueprints/Sound/SoundEffect/chicken.chicken" :`NewEnumerator4` "/Game/PLK_MR/Blueprints/Sound/SoundEffect/black.black" :`NewEnumerator5` "/Game/PLK_MR/Blueprints/Sound/SoundEffect/Green.Green" :!type "SoundBase Object Reference") (`self.K2_GetActorLocation`) (`KismetMathLibrary.FindLookAtRotation` (`SceneComponent.K2_GetComponentLocation` (`self.SkeletalMesh`)) (`SceneComponent.K2_GetComponentLocation` (`/Game/PLK_MR/Blueprints/BP_VRPawn.Camera` (`self.Player`)))) 1.0 1.0 0.0 "/Game/PLK_MR/Blueprints/Sound/3Dsound.3Dsound" null null null))))

(event `StartShooting`
  ;[1 1 1] Shooting enemy
  (switch `/Game/PLK_MR/Blueprints/Enum/Enum_EnemyTypes` (`self.EnemyTypes`)
    (:`NewEnumerator3`
      (set `self.bAttacking` true)
      (`KismetSystemLibrary.Delay` 1.0)
      (`|SpawnActorFromClass` "/Game/PLK_MR/Blueprints/BP_EnemyBullet.BP_EnemyBullet_C" (`KismetMathLibrary.MakeTransform` (`SceneComponent.K2_GetComponentLocation` (`self.ShootPoint`))) "Undefined" "MultiplyWithRoot" null (/ (`self.Atk`) 2) null)
      (`KismetSystemLibrary.Delay` 1.0)
      (`|SpawnActorFromClass` "/Game/PLK_MR/Blueprints/BP_EnemyBullet.BP_EnemyBullet_C" (`KismetMathLibrary.MakeTransform` (`SceneComponent.K2_GetComponentLocation` (`self.ShootPoint`))) "Undefined" "MultiplyWithRoot" null (/ (`self.Atk`) 2) null)
      (`KismetSystemLibrary.Delay` 2.54)
      (`self.StartShooting`))
    (:`NewEnumerator4`
      (set `self.bAttacking` true)
      (`KismetSystemLibrary.Delay` 2.0)
      (`|SpawnActorFromClass` "/Game/PLK_MR/Blueprints/BP_EnemyBullet.BP_EnemyBullet_C" (`KismetMathLibrary.MakeTransform` (`SceneComponent.K2_GetComponentLocation` (`self.ShootPoint`))) "Undefined" "MultiplyWithRoot" null (/ (`self.Atk`) 3) null)
      (`KismetSystemLibrary.Delay` 0.75)
      (`|SpawnActorFromClass` "/Game/PLK_MR/Blueprints/BP_EnemyBullet.BP_EnemyBullet_C" (`KismetMathLibrary.MakeTransform` (`SceneComponent.K2_GetComponentLocation` (`self.ShootPoint`))) "Undefined" "MultiplyWithRoot" null (/ (`self.Atk`) 3) null)
      (`KismetSystemLibrary.Delay` 0.75)
      (`|SpawnActorFromClass` "/Game/PLK_MR/Blueprints/BP_EnemyBullet.BP_EnemyBullet_C" (`KismetMathLibrary.MakeTransform` (`SceneComponent.K2_GetComponentLocation` (`self.ShootPoint`))) "Undefined" "MultiplyWithRoot" null (/ (`self.Atk`) 3) null)
      (`KismetSystemLibrary.Delay` 1.3)
      (set `self.bWaiting` true)
      (set `self.bAttacking` false)
      (`KismetSystemLibrary.Delay` 0.2)
      (set `self.bWaiting` false)
      (`KismetSystemLibrary.Delay` 4.0)
      (`self.StartShooting`))))

(event `Spawned`
  ;[1 1 1] Begin play
  (set `self.JustSpawned` false))

(event `self.ReceiveTick`
  (params (DeltaSeconds :type "Float (single-precision)"))
  (bind (_returnvalue_roll _returnvalue_pitch) (`KismetMathLibrary.BreakRotator` (`self.K2_GetActorRotation`)))
  (bind _returnvalue (* (`self.GetActorForwardVector`) (`self.Speed`) (`GameplayStatics.GetWorldDeltaSeconds`)))
  (bind _x (.x _returnvalue))
  (bind _y (.y _returnvalue))
  (bind (_returnvalue_roll_2 _returnvalue_pitch_2 _returnvalue_yaw) (`KismetMathLibrary.BreakRotator` (`KismetMathLibrary.FindLookAtRotation` (`SceneComponent.K2_GetComponentLocation` (`self.SkeletalMesh`)) (`SceneComponent.K2_GetComponentLocation` (`/Game/PLK_MR/Blueprints/BP_VRPawn.Camera` (`self.Player`))))))
  (bind _returnvalue_2 (`KismetMathLibrary.FindLookAtRotation` (`SceneComponent.K2_GetComponentLocation` (`self.Sphere`)) (`SceneComponent.K2_GetComponentLocation` (`/Game/PLK_MR/Blueprints/BP_VRPawn.Camera` (`self.Player`)))))
  (bind _yaw (.yaw _returnvalue_2))
  ;[1 1 1] Event tick
  (`|ExecutionSequence`
    (:`then_0`
      (switch `/Game/PLK_MR/Blueprints/Enum/Enum_EnemyTypes` (`self.EnemyTypes`)
        (:`NewEnumerator1`
          (`self.K2_SetActorRotation` (select `/Game/PLK_MR/Blueprints/Enum/Enum_EnemyTypes` (`self.EnemyTypes`) :`NewEnumerator0` _returnvalue_2 :`NewEnumerator1` _returnvalue_2 :`NewEnumerator2` (`KismetMathLibrary.MakeRotator` _returnvalue_roll _returnvalue_pitch _yaw) :`NewEnumerator3` _returnvalue_2 :`NewEnumerator4` _returnvalue_2 :`NewEnumerator5` (`KismetMathLibrary.MakeRotator` _returnvalue_roll _returnvalue_pitch _yaw)) true :!label _label_2))
        (:`NewEnumerator2`
          (goto _label_2))
        (:`NewEnumerator3`
          (`SceneComponent.K2_SetWorldRotation` (`self.SkeletalMesh`) (`KismetMathLibrary.MakeRotator` _returnvalue_roll_2 0.0 (- _returnvalue_yaw 90.0)) false false :!label _label_3))
        (:`NewEnumerator4`
          (goto _label_3))
        (:`NewEnumerator5`
          (goto _label_2))))
    (:`then_1`
      (if (`self.bAttacking`)
        _
        (elif (`self.bWaiting`)
          _
          (elif (`|EnumInequality` (`self.EnemyTypes`) "NewEnumerator3")
            (`self.K2_AddActorWorldOffset` (select `/Game/PLK_MR/Blueprints/Enum/Enum_EnemyTypes` (`self.EnemyTypes`) :`NewEnumerator0` _returnvalue :`NewEnumerator1` _returnvalue :`NewEnumerator2` (`KismetMathLibrary.MakeVector` _x _y) :`NewEnumerator3` _returnvalue :`NewEnumerator4` (`KismetMathLibrary.MakeVector` _x _y) :`NewEnumerator5` (`KismetMathLibrary.MakeVector` _x _y)) false true :!label _label_4)
            (`self.AnimationControler`)
            (elif (not (`self.bStop`))
              (goto _label_4))))))))

(event `AnimationControler`
  ;[1 1 1] Animation Controller
  (switch `/Game/PLK_MR/Blueprints/Enum/Enum_EnemyTypes` (`self.EnemyTypes`)
    (:`NewEnumerator1`
      (if (`self.DistanceDetecter` 50.0)
        (set `self.bAttacking` true)
        (`KismetSystemLibrary.Delay` 1.8)
        (`PrimitiveComponent.SetCollisionEnabled` (`self.PlayerDamage`) "QueryOnly")
        (`KismetSystemLibrary.Delay` 1.7)
        (`PrimitiveComponent.SetCollisionEnabled` (`self.PlayerDamage`) "NoCollision")
        (set `self.bWaiting` true)
        (set `self.bAttacking` false)
        (`KismetSystemLibrary.Delay` 0.1)
        (set `self.bWaiting` false)))
    (:`NewEnumerator2`
      (if (`self.DistanceDetecter` 50.0)
        (set `self.bAttacking` true)
        (`KismetSystemLibrary.Delay` 0.6)
        (`PrimitiveComponent.SetCollisionEnabled` (`self.PlayerDamage`) "QueryOnly")
        (`KismetSystemLibrary.Delay` 1.4)
        (`PrimitiveComponent.SetCollisionEnabled` (`self.PlayerDamage`) "NoCollision")
        (set `self.bWaiting` true)
        (set `self.bAttacking` false)
        (`KismetSystemLibrary.Delay` 1.0)
        (set `self.bWaiting` false)))
    (:`NewEnumerator5`
      (if (`self.DistanceDetecter` 100.0)
        (set `self.bAttacking` true)
        (`KismetSystemLibrary.Delay` 0.9)
        (`PrimitiveComponent.SetCollisionEnabled` (`self.PlayerDamage`) "QueryOnly")
        (`KismetSystemLibrary.Delay` 0.1)
        (`PrimitiveComponent.SetCollisionEnabled` (`self.PlayerDamage`) "NoCollision")
        (`KismetSystemLibrary.Delay` 0.8)
        (`PrimitiveComponent.SetCollisionEnabled` (`self.PlayerDamage`) "QueryOnly")
        (`KismetSystemLibrary.Delay` 0.2)
        (`PrimitiveComponent.SetCollisionEnabled` (`self.PlayerDamage`) "NoCollision")
        (`KismetSystemLibrary.Delay` 1.6)
        (set `self.bWaiting` true)
        (set `self.bAttacking` false)
        (`KismetSystemLibrary.Delay` 3.0)
        (set `self.bWaiting` false)))))

(event `Damaged`
  (params (Damage :type Integer) (bIsLaser :type Boolean))
  (bind _playerstate (`/Game/PLK_MR/Library/BP_FunctionLibrary.GetOwningPlayerState`))
  (bind _returnvalue (`self.K2_GetActorLocation`))
  ;[1 1 1] Damaged
  (if bIsLaser
    (`/Engine/EditorBlueprintResources/StandardMacros.DoOnce` false :!label _label_5
      (:`Completed`
        (`|ExecutionSequence`
          (:`then_0`
            _)
          (:`then_1`
            (`KismetSystemLibrary.Delay` 0.5)
            (goto _label_5 :!via `Reset`))))))
  (bind _output_get (set `self.Hp` (- (`self.Hp`) Damage)))
  (`|ExecutionSequence`
    (:`then_0`
      (if (<= _output_get 0)
        (`|ExecutionSequence`
          (:`then_0`
            (`/Game/PLK_MR/GameModes/SharedSpaces/BP_PLKPlayerState.Update_PlayerCoins` _playerstate (select `/Game/PLK_MR/Blueprints/Enum/Enum_EnemyLevels` (`self.EnemyLevel`) :`NewEnumerator0` 2 :`NewEnumerator1` 5 :`NewEnumerator2` 8))
            (`/Game/PLK_MR/GameModes/SharedSpaces/BP_PLKPlayerState.Update_PlayerKills` _playerstate 1)
            (if (== (`KismetMathLibrary.RandomIntegerInRange` 1 7) 5)
              (`|SpawnActorFromClass` "/Game/PLK_MR/Blueprints/BP_Chest.BP_Chest_C" (`KismetMathLibrary.MakeTransform` (`self.K2_GetActorLocation`) (`KismetMathLibrary.FindLookAtRotation` (`self.K2_GetActorLocation`) (`SceneComponent.K2_GetComponentLocation` (`/Game/PLK_MR/Blueprints/BP_VRPawn.Camera` (`/Game/PLK_MR/Library/BP_FunctionLibrary.Get VR Pawn`))))) "Undefined" "MultiplyWithRoot" null null)))
          (:`then_1`
            (`self.DestroySelf`)))))
    (:`then_1`
      (`|SpawnActorFromClass` "/Game/PLK_MR/Blueprints/Widget/BP_Damaged.BP_Damaged_C" (`KismetMathLibrary.MakeTransform` _returnvalue) "Undefined" "MultiplyWithRoot" null (`KismetStringLibrary.Conv_IntToString` Damage) null)
      (`GameplayStatics.PlaySoundAtLocation` "/Game/PLK_MR/Blueprints/Sound/enemyhurt.enemyhurt" _returnvalue (struct) 1.0 1.0 0.0 "/Game/PLK_MR/Blueprints/Sound/3Dsound.3Dsound" null null null))))

(event `self.HitCollider.OnComponentBeginOverlap`
  (params (OverlappedComponent :type "PrimitiveComponent Object Reference") (OtherActor :type "Actor Object Reference") (OtherComp :type "PrimitiveComponent Object Reference") (OtherBodyIndex :type Integer) (bFromSweep :type Boolean) (SweepResult :type "HitResult Structure (by ref)"))
  ;[1 1 1] Overlap
  (`|ExecutionSequence`
    (:`then_0`
      (switch `/Game/PLK_MR/Blueprints/Enum/Enum_EnemyTypes` (`self.EnemyTypes`)))
    (:`then_1`
      (switch `/Game/PLK_MR/Blueprints/Enum/Enum_EnemyTypes` (`self.EnemyTypes`)
        (:`NewEnumerator4`
          (cast `/Game/PLK_MR/Blueprints/BP_Room` OtherActor)
          (if (not (`self.JustSpawned`))
            (`self.ReverseRotation`)))))))

(event `ReverseRotation`
  (bind (_returnvalue_roll _returnvalue_pitch _returnvalue_yaw) (`KismetMathLibrary.BreakRotator` (`KismetMathLibrary.FindLookAtRotation` (`self.K2_GetActorLocation`) (* (`self.GetActorForwardVector`) -200.0))))
  ;[1 1 1] Change rotation when hit wall
  (`self.K2_SetActorRotation` (`KismetMathLibrary.MakeRotator` 0.0 0.0 (+ _returnvalue_yaw (`KismetMathLibrary.RandomFloatInRange` -40.0 40.0))) true))

(event `DestroySelf`
  (`self.K2_DestroyActor`))

(event `self.PlayerDamage.OnComponentBeginOverlap`
  (params (OverlappedComponent :type "PrimitiveComponent Object Reference") (OtherActor :type "Actor Object Reference") (OtherComp :type "PrimitiveComponent Object Reference") (OtherBodyIndex :type Integer) (bFromSweep :type Boolean) (SweepResult :type "HitResult Structure (by ref)"))
  ;[1 1 1] Damage player when hit collider hit
  (bind _asbp_vrpawn (cast `/Game/PLK_MR/Blueprints/BP_VRPawn` OtherActor))
  (`/Game/PLK_MR/Blueprints/BP_VRPawn.DamagePlayer` _asbp_vrpawn (`self.Atk`))
  (`PrimitiveComponent.SetCollisionEnabled` (`self.PlayerDamage`) "NoCollision"))

(fn `DistanceDetecter`
  (params (Distance :type "Float (double-precision)"))
  (returns (`PlayerInDistance?` :type Boolean) (ActualDistance :type "Float (double-precision)"))
  (bind (_returnvalue_x _returnvalue_y) (`KismetMathLibrary.BreakVector` (`self.K2_GetActorLocation`)))
  (bind (_returnvalue_x_2 _returnvalue_y_2) (`KismetMathLibrary.BreakVector` (`SceneComponent.K2_GetComponentLocation` (`/Game/PLK_MR/Blueprints/BP_VRPawn.Camera` (`self.Player`)))))
  (bind _returnvalue (`KismetMathLibrary.Vector_Distance` (`KismetMathLibrary.MakeVector` _returnvalue_x _returnvalue_y) (`KismetMathLibrary.MakeVector` _returnvalue_x_2 _returnvalue_y_2)))
  (return (<= _returnvalue Distance) _returnvalue))

(fn `Shooting`
  (switch `/Game/PLK_MR/Blueprints/Enum/Enum_EnemyTypes` (`self.EnemyTypes`)))

(fn `UserConstructionScript`)