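; BP_Chest is a reward chest actor for VR with a world-space widget that floats above its cube and turns toward the VR pawn's camera every tick.
; On BeginPlay it registers itself as the widget's owner and keeps the Niagara reward effect off.
; OpenChest takes a success flag: success removes the widget and plays the effect briefly before destroying the chest, while failure destroys it immediately.
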(event `self.ReceiveBeginPlay`
  (set `/Game/PLK_MR/Blueprints/Widget/WBP_ChestWidget.OwnerChest` self (cast `/Game/PLK_MR/Blueprints/Widget/WBP_ChestWidget` (`WidgetComponent.GetWidget` (`self.Widget`)) :!pure true))
  (`ActorComponent.Deactivate` (`self.NS_Chest_reward`)))

(event `OpenChest`
  (params (`bSuccess?` :type Boolean))
  (bind _ns_chest_reward (`self.NS_Chest_reward`))
  (bind _widget (`self.Widget`))
  (if `bSuccess?`
    (`PrimitiveComponent.SetCollisionEnabled` _widget "NoCollision")
    (`|ExecutionSequence`
      (:`then_0`
        (`WidgetComponent.SetWidget` _widget null))
      (:`then_1`
        (`ActorComponent.Activate` _ns_chest_reward true)
        (`KismetSystemLibrary.Delay` 2.0)
        (`ActorComponent.Deactivate` _ns_chest_reward)
        (`self.K2_DestroyActor`)))
    (else
      (`self.K2_DestroyActor`))))

(event `self.ReceiveTick`
  (params (DeltaSeconds :type "Float (single-precision)"))
  ;[1 1 1] Widget look at
  (`SceneComponent.K2_SetWorldRotation` (`self.Widget`) (`KismetMathLibrary.FindLookAtRotation` (`SceneComponent.K2_GetComponentLocation` (`self.Widget`)) (`SceneComponent.K2_GetComponentLocation` (`/Game/PLK_MR/Blueprints/BP_VRPawn.Camera` (`/Game/PLK_MR/Library/BP_FunctionLibrary.Get VR Pawn`)))) false false)
  (`SceneComponent.K2_SetWorldLocation` (`self.Widget`) (+ (`SceneComponent.K2_GetComponentLocation` (`self.Cube`)) (0.0 0.0 100.0)) false true))

(fn `UserConstructionScript`
  (`SceneComponent.K2_SetWorldLocation` (`self.Widget`) (+ (`SceneComponent.K2_GetComponentLocation` (`self.Cube`)) (25.0 0.0 100.0)) false true))