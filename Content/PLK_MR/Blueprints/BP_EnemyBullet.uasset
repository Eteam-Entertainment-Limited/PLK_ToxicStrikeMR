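; BP_EnemyBullet is an enemy projectile aimed at the VR player that damages them on contact.
; On spawn it turns its collision sphere toward the VR pawn's camera, then launches it with a one-time Speed-scaled velocity impulse along actor forward, with no later homing.
; Overlapping a BP_VRPawn calls DamagePlayer with Atk and destroys the bullet; other overlaps are ignored, and a timer destroys it after a short lifetime.
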(event `self.ReceiveBeginPlay`
  ;[1 1 1] Begin play
  (`SceneComponent.K2_SetWorldRotation` (`self.SphereCollision`) (`KismetMathLibrary.FindLookAtRotation` (`self.K2_GetActorLocation`) (`SceneComponent.K2_GetComponentLocation` (`/Game/PLK_MR/Blueprints/BP_VRPawn.Camera` (`/Game/PLK_MR/Library/BP_FunctionLibrary.Get VR Pawn`)))) false false)
  (`PrimitiveComponent.AddImpulse` (`self.SphereCollision`) (* (`self.GetActorForwardVector`) 1000.0 (`self.Speed`)) "None" true)
  (`KismetSystemLibrary.K2_SetTimerDelegate` (delegate `CustomEvent`) 5.0))

(event `CustomEvent`
  ;[1 1 1] Begin play
  (`self.K2_DestroyActor`))

(event `self.Sphere.OnComponentBeginOverlap`
  (params (OverlappedComponent :type "PrimitiveComponent Object Reference") (OtherActor :type "Actor Object Reference") (OtherComp :type "PrimitiveComponent Object Reference") (OtherBodyIndex :type Integer) (bFromSweep :type Boolean) (SweepResult :type "HitResult Structure (by ref)"))
  ;[1 1 1] Damage
  (`|ExecutionSequence`
    (:`then_0`
      (bind _asbp_vrpawn (cast `/Game/PLK_MR/Blueprints/BP_VRPawn` OtherActor))
      (`/Game/PLK_MR/Blueprints/BP_VRPawn.DamagePlayer` _asbp_vrpawn (`self.Atk`))
      (`self.K2_DestroyActor`))))

(fn `UserConstructionScript`)