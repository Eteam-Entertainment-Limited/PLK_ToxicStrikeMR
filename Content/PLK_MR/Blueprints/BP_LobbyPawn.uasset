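; BP_LobbyPawn is the lobby player pawn, which lets the player navigate and select main menu items through Enhanced Input.
; BeginPlay adds the base mapping context and calls the game instance's PlaySound, while input actions forward to LobbyMenuManagerComponent.
; The construction script hands that component its menu attachment point and session manager.
; A motion-controller laser pointer, using a sphere trace and spline mesh, exists but is disconnected from the empty Tick.
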(event `self.ReceiveBeginPlay`
  (bind _asplayer_controller (cast `PlayerController` (`self.GetController`)))
  (`EnhancedInputSubsystemInterface.AddMappingContext` (pcsubsystem `EnhancedInputLocalPlayerSubsystem` _asplayer_controller) "/Game/PLK_MR/Inputs/Mapppings/IMC_Base.IMC_Base" 0 (struct))
  (bind _asgi_game_level (cast `/Game/Blueprints/GI_GameLevel` (`GameplayStatics.GetGameInstance`)))
  (`/Game/Blueprints/GI_GameLevel.playSound` _asgi_game_level))

(event `EnhancedInput|/Game/PLK_MR/Inputs/Actions/IA_SelectMainMenuItem`
  (params (ActionValue :type "Float (double-precision)") (ElapsedSeconds :type "Float (double-precision)") (TriggeredSeconds :type "Float (double-precision)") (InputAction :type "InputAction Object Reference" :default "/Game/PLK_MR/Inputs/Actions/IA_SelectMainMenuItem.IA_SelectMainMenuItem"))
  ;[1 1 1 1 95] USER INPUT
  ;;[1 1 1] Menu Selection
  (:`Triggered`
    (`/Game/PLK_MR/Blueprints/Components/BP_LobbyMenuManager.Select Main Menu Item` (`self.LobbyMenuManagerComponent`))))

(event `EnhancedInput|/Game/PLK_MR/Inputs/Actions/IA_MenuSelectionUpDown`
  (params (ActionValue :type "Float (double-precision)") (ElapsedSeconds :type "Float (double-precision)") (TriggeredSeconds :type "Float (double-precision)") (InputAction :type "InputAction Object Reference" :default "/Game/PLK_MR/Inputs/Actions/IA_MenuSelectionUpDown.IA_MenuSelectionUpDown"))
  (bind _lobbymenumanagercomponent (`self.LobbyMenuManagerComponent`))
  ;[1 1 1 1 95] USER INPUT
  ;;[1 1 1] Menu Navigation
  (:`Triggered`
    (if (> ActionValue 0.0)
      (`/Game/PLK_MR/Blueprints/Components/BP_LobbyMenuManager.Menu Selection Up` _lobbymenumanagercomponent)
      (else
        (`/Game/PLK_MR/Blueprints/Components/BP_LobbyMenuManager.Menu Selection Down` _lobbymenumanagercomponent)))))

(event `self.ReceiveTick`
  (params (DeltaSeconds :type "Float (single-precision)"))
  ;[1 1 1] Hover Anchor
)

(fn `UpdateSplineMesh`
  (bind _spline (`self.Spline`))
  (bind (_location _tangent) (`SplineComponent.GetLocationAndTangentAtSplinePoint` _spline 1 "Local"))
  (bind (_location_2 _tangent_2) (`SplineComponent.GetLocationAndTangentAtSplinePoint` _spline 0 "Local"))
  (`SplineMeshComponent.SetStartAndEnd` (`self.SplineMesh`) _location_2 _tangent_2 _location _tangent true))

(fn `UserConstructionScript`
  (bind _lobbymenumanagercomponent (`self.LobbyMenuManagerComponent`))
  (set `/Game/PLK_MR/Blueprints/Components/BP_LobbyMenuManager.MainMenuPositioner` (`self.MainMenuAttachmentPoint`) _lobbymenumanagercomponent)
  (set `/Game/PLK_MR/Blueprints/Components/BP_LobbyMenuManager.Session Manager` (`self.SessionManagerComponent`) _lobbymenumanagercomponent))