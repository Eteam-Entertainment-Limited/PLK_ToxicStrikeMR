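; BP_Room is an adjustable four-wall room that serves as the spawn arena for enemies and the boss.
; Wall spacing, height and room elevation load from the "WallDetail" save, change through step events, and drive the wall layout, also previewed in construction.
; Walls hide after BeginPlay.
; A level-paced looping timer spawns enemies along Front, Left or Right, with type and height set by player-state level, randomized during Boss.
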(event `Room_Changing`
  (bind (_returnvalue_x _returnvalue_y) (`KismetMathLibrary.BreakVector` (`self.K2_GetActorLocation`)))
  ;[1 1 1] Room Setting
  (`|ExecutionSequence`
    (:`then_0`
      (`SceneComponent.K2_SetRelativeLocation` (`self.Front`) (`KismetMathLibrary.MakeVector` (/ (`self.WallXDistance`) 2.0) 0.0 (* (`self.WallHeightScaling`) 50.0)) false false)
      (`SceneComponent.K2_SetRelativeLocation` (`self.Back`) (`KismetMathLibrary.MakeVector` (* (/ (`self.WallXDistance`) 2.0) -1.0) 0.0 (* (`self.WallHeightScaling`) 50.0)) false false))
    (:`then_1`
      (`SceneComponent.K2_SetRelativeLocation` (`self.Right`) (`KismetMathLibrary.MakeVector` 0.0 (/ (`self.WallYDistance`) 2.0) (* (`self.WallHeightScaling`) 50.0)) false false)
      (`SceneComponent.K2_SetRelativeLocation` (`self.Left`) (`KismetMathLibrary.MakeVector` 0.0 (* (/ (`self.WallYDistance`) 2.0) -1.0) (* (`self.WallHeightScaling`) 50.0)) false false))
    (:`then_2`
      (`SceneComponent.SetRelativeScale3D` (`self.Front`) (`KismetMathLibrary.MakeVector` (/ (`self.WallYDistance`) 100.0) (`self.WallHeightScaling`) 1.0))
      (`SceneComponent.SetRelativeScale3D` (`self.Back`) (`KismetMathLibrary.MakeVector` (/ (`self.WallYDistance`) 100.0) (`self.WallHeightScaling`) 1.0))
      (`SceneComponent.SetRelativeScale3D` (`self.Right`) (`KismetMathLibrary.MakeVector` (/ (`self.WallXDistance`) 100.0) (`self.WallHeightScaling`) 1.0))
      (`SceneComponent.SetRelativeScale3D` (`self.Left`) (`KismetMathLibrary.MakeVector` (/ (`self.WallXDistance`) 100.0) (`self.WallHeightScaling`) 1.0)))
    (:`then_3`
      (`self.K2_SetActorLocation` (`KismetMathLibrary.MakeVector` _returnvalue_x _returnvalue_y (`self.RoomHeight`))))))

(event `self.ReceiveBeginPlay`
  (`KismetSystemLibrary.Delay` 1.0)
  (`|ExecutionSequence`
    (:`then_0`
      (bind (_success_ _wallstrans) (`/Game/PLK_MR/Library/BP_FunctionLibrary.Load Game` "WallDetail"))
      (if _success_
        (`self.LoadAllWallTrans` _wallstrans)))
    (:`then_1`
      (`self.Wall Showing Control` true))))

(event `DistAdd_X`
  ;[1 1 1] Custom Wall
  (set `self.WallXDistance` (+ (`self.WallXDistance`) 1.0))
  (`self.Room_Changing` :!label _label))

(event `LoadAllWallTrans`
  (params (WallsTrans :type "Array of Float (double-precision)"))
  (for (_array_element _array_index) WallsTrans
    (switch `int` _array_index
      (:`0`
        (set `self.WallXDistance` _array_element))
      (:`1`
        (set `self.WallYDistance` _array_element))
      (:`2`
        (set `self.WallHeightScaling` _array_element))
      (:`3`
        (set `self.RoomHeight` _array_element))))
  (`self.Room_Changing`))

(event `DistMinus_X`
  ;[1 1 1] Custom Wall
  (set `self.WallXDistance` (- (`self.WallXDistance`) 1.0))
  (goto _label))

(event `DistAdd_Y`
  ;[1 1 1] Custom Wall
  (set `self.WallYDistance` (+ (`self.WallYDistance`) 1.0))
  (goto _label))

(event `DistMinus_Y`
  ;[1 1 1] Custom Wall
  (set `self.WallYDistance` (- (`self.WallYDistance`) 1.0))
  (goto _label))

(event `Wall Showing Control`
  (params (bDisappear :type Boolean))
  (`SceneComponent.SetHiddenInGame` (`self.Front`) bDisappear false)
  (`SceneComponent.SetHiddenInGame` (`self.Back`) bDisappear false)
  (`SceneComponent.SetHiddenInGame` (`self.Left`) bDisappear false)
  (`SceneComponent.SetHiddenInGame` (`self.Right`) bDisappear false))

(event `Add_HeightScaling`
  ;[1 1 1] Custom Wall
  (set `self.WallHeightScaling` (+ (`self.WallHeightScaling`) 0.025))
  (`self.Room_Changing` :!label _label_2))

(event `StartSpawningEnemies`
  (params (Levels :type "/Game/PLK_MR/Blueprints/Structure/Enum_GameLevels Enum" :default "NewEnumerator6"))
  (`KismetSystemLibrary.K2_ClearAndInvalidateTimerHandle` (`self.SpawnTimer`))
  (bind _returnvalue (`KismetSystemLibrary.K2_SetTimer` null "SpawnNewEnemy" (select `/Game/PLK_MR/Blueprints/Structure/Enum_GameLevels` Levels :`NewEnumerator0` 3.0 :`NewEnumerator1` 3.0 :`NewEnumerator2` 2.0 :`NewEnumerator3` 2.0 :`NewEnumerator5` 2.0 :!type "Float (single-precision)") true))
  (set `self.SpawnTimer` _returnvalue))

(event `Minus_HeightScaling`
  ;[1 1 1] Custom Wall
  (set `self.WallHeightScaling` (- (`self.WallHeightScaling`) 0.025))
  (goto _label_2))

(event `Add_RoomHeight`
  ;[1 1 1] Custom Wall
  (set `self.RoomHeight` (+ (`self.RoomHeight`) 0.5))
  (`self.Room_Changing` :!label _label_3))

(event `StopSpawning`
  (bind _spawntimer (`self.SpawnTimer`))
  (if (`KismetSystemLibrary.K2_IsTimerActiveHandle` _spawntimer)
    (`KismetSystemLibrary.K2_ClearAndInvalidateTimerHandle` _spawntimer)))

(event `Minus_RoomHeight`
  ;[1 1 1] Custom Wall
  (set `self.RoomHeight` (- (`self.RoomHeight`) 0.5))
  (goto _label_3))

(event `SpawnBoss`
  (bind (_relativelocation_x _relativelocation_y) (`KismetMathLibrary.BreakVector` (`SceneComponent.RelativeLocation` (`self.Front`))))
  (bind _returnvalue (`|SpawnActorFromClass` "/Game/PLK_MR/Blueprints/BP_Boss.BP_Boss_C" (`KismetMathLibrary.MakeTransform` (`KismetMathLibrary.MakeVector` _relativelocation_x _relativelocation_y)) "Undefined" "MultiplyWithRoot" null null null))
  (set `/Game/PLK_MR/GameModes/SharedSpaces/BP_PLKPlayerState.BossRef` _returnvalue (`/Game/PLK_MR/Library/BP_FunctionLibrary.GetOwningPlayerState`))
  (`self.StartSpawningEnemies` "NewEnumerator5"))

(event `Selected Wall Scale Y`
  ;[1 1 1] Custom Wall
)

(event `Selected Wall Scale Down Y`
  ;[1 1 1] Custom Wall
)

(event `Selected Wall Scale Z`
  ;[1 1 1] Custom Wall
)

(event `Selected Wall Scale Down Z`
  ;[1 1 1] Custom Wall
)

(fn `GetAllWallsTrans`
  (returns (WallsTrans :type "Array of Float (double-precision)"))
  (return (`|MakeArray` (`self.WallXDistance`) (`self.WallYDistance`) (`self.WallHeightScaling`) (`self.RoomHeight`))))

(fn `SpawnNewEnemy`
  (locals (TempRandomNumber :type Integer) (TempRandomEnemy :type "/Game/PLK_MR/Blueprints/Structure/Enum_EnemyType Enum"))
  (bind _returnvalue (select `int` (`local.TempRandomNumber`) :`0` (`self.Front`) :`1` (`self.Left`) :`2` (`self.Right`) :`3` (`self.Back`)))
  (bind _returnvalue_2 (`SceneComponent.K2_GetComponentLocation` _returnvalue))
  (bind _returnvalue_3 (select `/Game/PLK_MR/Blueprints/Structure/Enum_GameLevels` (`/Game/PLK_MR/GameModes/SharedSpaces/BP_PLKPlayerState.Level` (`/Game/PLK_MR/Library/BP_FunctionLibrary.GetOwningPlayerState`)) :`NewEnumerator6` "NewEnumerator5" :`NewEnumerator0` "NewEnumerator5" :`NewEnumerator1` "NewEnumerator0" :`NewEnumerator2` "NewEnumerator1" :`NewEnumerator3` "NewEnumerator2" :`NewEnumerator5` (`local.TempRandomEnemy`) :`NewEnumerator4` "NewEnumerator5"))
  (bind (_relativescale3d_x _relativescale3d_y) (`KismetMathLibrary.BreakVector` (`SceneComponent.RelativeScale3D` _returnvalue)))
  (bind (_relativescale3d_x_2 _relativescale3d_y_2) (`KismetMathLibrary.BreakVector` (`SceneComponent.RelativeScale3D` _returnvalue)))
  (bind _y (.y _returnvalue_2))
  (bind _x (.x _returnvalue_2))
  (bind _z (.z _returnvalue_2))
  (bind _returnvalue_4 (* 40.0 _relativescale3d_x))
  (bind _returnvalue_5 (* 40.0 _relativescale3d_y))
  (bind _returnvalue_6 (* 40.0 _relativescale3d_x_2))
  (bind _returnvalue_7 (* 40.0 _relativescale3d_y_2))
  (bind _returnvalue_8 (* 40.0 _relativescale3d_x_2))
  (bind _returnvalue_9 (* 40.0 _relativescale3d_y_2))
  (bind _returnvalue_10 (* 40.0 _relativescale3d_y_2))
  (bind _returnvalue_11 (* 40.0 _relativescale3d_x_2))
  (bind _returnvalue_12 (select `int` (`local.TempRandomNumber`) :`0` (`KismetMathLibrary.MakeVector` (.x _returnvalue_2) (+ (.y _returnvalue_2) (`KismetMathLibrary.RandomFloatInRange` (* _returnvalue_8 -1.0) _returnvalue_8)) (+ (.z _returnvalue_2) (`KismetMathLibrary.RandomFloatInRange` (* _returnvalue_9 -1.0) _returnvalue_9))) :`1` (`KismetMathLibrary.MakeVector` (+ _x (`KismetMathLibrary.RandomFloatInRange` (* _returnvalue_6 -1.0) _returnvalue_6)) _y (+ _z (`KismetMathLibrary.RandomFloatInRange` (* _returnvalue_7 -1.0) _returnvalue_7))) :`2` (`KismetMathLibrary.MakeVector` (+ _x (`KismetMathLibrary.RandomFloatInRange` (* _returnvalue_11 -1.0) _returnvalue_11)) _y (+ _z (`KismetMathLibrary.RandomFloatInRange` (* _returnvalue_10 -1.0) _returnvalue_10))) :`3` (`KismetMathLibrary.MakeVector` _x (+ (.y _returnvalue_2) (`KismetMathLibrary.RandomFloatInRange` (* _returnvalue_4 -1.0) _returnvalue_4)) (+ (.z _returnvalue_2) (`KismetMathLibrary.RandomFloatInRange` (* _returnvalue_5 -1.0) _returnvalue_5)))))
  (bind _x_2 (.x _returnvalue_12))
  (bind _y_2 (.y _returnvalue_12))
  (set `local.TempRandomNumber` (`KismetMathLibrary.RandomIntegerInRange` 0 2))
  (set `local.TempRandomEnemy` (select `int` (`KismetMathLibrary.RandomIntegerInRange` 0 2) :`0` "NewEnumerator0" :`1` "NewEnumerator1" :`2` "NewEnumerator2" :!type "/Game/PLK_MR/Blueprints/Structure/Enum_EnemyType Enum"))
  (`|SpawnActorFromClass` "/Game/PLK_MR/Blueprints/BP_BaseEnemy.BP_BaseEnemy_C" (`KismetMathLibrary.MakeTransform` (select `/Game/PLK_MR/Blueprints/Structure/Enum_EnemyType` _returnvalue_3 :`NewEnumerator5` _returnvalue_12 :`NewEnumerator0` _returnvalue_12 :`NewEnumerator1` (`KismetMathLibrary.MakeVector` _x_2 _y_2 10.0) :`NewEnumerator2` (`KismetMathLibrary.MakeVector` _x_2 _y_2 (`KismetMathLibrary.RandomFloatInRange` 180.0 230.0))) (select `int` (`local.TempRandomNumber`) :`0` (struct :`Yaw` -180.0) :`1` (struct :`Yaw` 90.0) :`2` (struct :`Yaw` -90.0) :`3` (struct) :!type "Rotator Structure")) "Undefined" "MultiplyWithRoot" null _returnvalue_3 null))

(fn `UserConstructionScript`
  (bind (_returnvalue_x _returnvalue_y) (`KismetMathLibrary.BreakVector` (`self.K2_GetActorLocation`)))
  (`|ExecutionSequence`
    (:`then_0`
      (`SceneComponent.K2_SetRelativeLocation` (`self.Front`) (`KismetMathLibrary.MakeVector` (/ (`self.WallXDistance`) 2.0) 0.0 (* (`self.WallHeightScaling`) 50.0)) false false)
      (`SceneComponent.K2_SetRelativeLocation` (`self.Back`) (`KismetMathLibrary.MakeVector` (* (/ (`self.WallXDistance`) 2.0) -1.0) 0.0 (* (`self.WallHeightScaling`) 50.0)) false false))
    (:`then_1`
      (`SceneComponent.K2_SetRelativeLocation` (`self.Right`) (`KismetMathLibrary.MakeVector` 0.0 (/ (`self.WallYDistance`) 2.0) (* (`self.WallHeightScaling`) 50.0)) false false)
      (`SceneComponent.K2_SetRelativeLocation` (`self.Left`) (`KismetMathLibrary.MakeVector` 0.0 (* (/ (`self.WallYDistance`) 2.0) -1.0) (* (`self.WallHeightScaling`) 50.0)) false false))
    (:`then_2`
      (`SceneComponent.SetRelativeScale3D` (`self.Front`) (`KismetMathLibrary.MakeVector` (/ (`self.WallYDistance`) 100.0) (`self.WallHeightScaling`) 1.0))
      (`SceneComponent.SetRelativeScale3D` (`self.Back`) (`KismetMathLibrary.MakeVector` (/ (`self.WallYDistance`) 100.0) (`self.WallHeightScaling`) 1.0))
      (`SceneComponent.SetRelativeScale3D` (`self.Right`) (`KismetMathLibrary.MakeVector` (/ (`self.WallXDistance`) 100.0) (`self.WallHeightScaling`) 1.0))
      (`SceneComponent.SetRelativeScale3D` (`self.Left`) (`KismetMathLibrary.MakeVector` (/ (`self.WallXDistance`) 100.0) (`self.WallHeightScaling`) 1.0)))
    (:`then_3`
      (`self.K2_SetActorLocation` (`KismetMathLibrary.MakeVector` _returnvalue_x _returnvalue_y (`self.RoomHeight`))))))