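; VR gun actor whose GunType makes it a handgun, shotgun, sniper, machine gun or laser gun.
; Projectile types spawn BP_Bullet with DoOnce-gated fire, updating the ammo widget, haptics and timed reload; GodMode skips ammo use.
; The laser sphere-traces to damage enemies, hit boss weakpoints and select quiz answers, updating a spline endpoint.
; A timeline flies remotely grabbed guns to the controller, and a looping timer teleports strayed guns near the player.
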(event `CustomEvent`
  ;[1 1 1] Begin play
  (`ActorComponent.Activate` (`self.N_BulletShoot`) true))

(event `self.ReceiveBeginPlay`
  (bind _spline (`self.Spline`))
  ;[1 1 1] Begin play
  (`|ExecutionSequence`
    (:`then_0`
      (`NiagaraComponent.SetAsset` (`self.N_BulletShoot`) (select `/Game/PLK_MR/Blueprints/Enum/Enum_GunType` (`self.GunType`) :`NewEnumerator0` "/Game/PLK_MR/VFX/NS_Gun1_MuzzleFlash.NS_Gun1_MuzzleFlash" :`NewEnumerator1` "/Game/PLK_MR/VFX/NS_Gun2_MuzzleFlash.NS_Gun2_MuzzleFlash" :`NewEnumerator2` "/Game/PLK_MR/VFX/NS_Gun2_MuzzleFlash.NS_Gun2_MuzzleFlash" :`NewEnumerator3` "/Game/PLK_MR/VFX/NS_Gun3_MuzzleFlash.NS_Gun3_MuzzleFlash" :`NewEnumerator4` "/Game/PLK_MR/VFX/NS_beam.NS_beam" :!type "NiagaraSystem Object Reference") true)
      (`ActorComponent.Deactivate` (`self.N_BulletShoot`))
      (`ActorComponent.Deactivate` (`self.NS_Gunbeam`))
      (`SplineComponent.SetLocationAtSplinePoint` _spline 1 (`SplineComponent.GetLocationAtSplinePoint` _spline 0 "World") "World" true)
      (`self.UpdateSplineMesh`)
      (bind _output_get (set `self.MaxAmmo` (select `/Game/PLK_MR/Blueprints/Enum/Enum_GunType` (`self.GunType`) :`NewEnumerator0` 12 :`NewEnumerator1` 8 :`NewEnumerator2` 15 :`NewEnumerator3` 50)))
      (set `self.Ammo` _output_get)
      (`self.SetAmmoText`)
      (`KismetSystemLibrary.K2_SetTimerDelegate` (delegate `CheckDistance`) 2.0 true))))

(event `CheckDistance`
  (bind (_relativelocation_x _relativelocation_y _relativelocation_z) (`KismetMathLibrary.BreakVector` (`SceneComponent.RelativeLocation` (`/Game/PLK_MR/Blueprints/BP_VRPawn.Camera` (`/Game/PLK_MR/Library/BP_FunctionLibrary.Get VR Pawn`)))))
  ;[1 1 1] Begin play
  (if (not (`self.DistanceDetecter` 1000.0))
    (`PrimitiveComponent.SetSimulatePhysics` (`self.Body`) false)
    (`self.K2_SetActorLocation` (`KismetMathLibrary.MakeVector` (+ _relativelocation_x 50.0) _relativelocation_y _relativelocation_z) false true)
    (`PrimitiveComponent.SetSimulatePhysics` (`self.Body`) true)))

(event `self.ReceiveTick`
  (params (DeltaSeconds :type "Float (single-precision)"))
  ;[1 1 1] Event tick
  (bind _lasersound (`self.LaserSound`)
    (:`then`
      (`SceneComponent.K2_SetWorldLocation` _lasersound (`self.K2_GetActorLocation`) false true))
    (:`else`)))

(event `Grabbing_By_Player`
  (params (ControllerRef :type "MotionControllerComponent Object Reference") (HandType :type "EControllerHand Enum" :default "Left"))
  (bind (_originalrotation_roll _originalrotation_pitch _originalrotation_yaw) (`KismetMathLibrary.BreakRotator` (`self.OriginalRotation`)))
  (bind (_location_offset_x _location_offset_y _location_offset_z) (`KismetMathLibrary.BreakVector` (`self.Location Offset`)))
  (bind (_returnvalue_x _returnvalue_y _returnvalue_z) (`KismetMathLibrary.BreakVector` (- (`self.Controller Location`) (`self.Original Location`))))
  (bind (_returnvalue_x_2 _returnvalue_y_2 _returnvalue_z_2) (`KismetMathLibrary.BreakVector` (- (`SceneComponent.K2_GetComponentLocation` ControllerRef) (`self.Original Location`))))
  ;[1 1 1] Grab Gun from far away
  (if (`/Game/PLK_MR/Blueprints/GrabComponent.bIsHeld` (`self.GrabComponent`))
    (`/Game/PLK_MR/Blueprints/BP_VRPawn.CatchGun` (cast `/Game/PLK_MR/Blueprints/BP_VRPawn` (`ActorComponent.GetOwner` ControllerRef) :!pure true) null HandType)
    (else
      (set `self.Grabbing` true)
      (set `self.Controller Location` (`SceneComponent.K2_GetComponentLocation` ControllerRef))
      (set `self.Original Location` (`self.K2_GetActorLocation`))
      (set `self.OriginalRotation` (`self.K2_GetActorRotation`))
      (`PrimitiveComponent.SetSimulatePhysics` (`self.Body`) false)
      (set `self.isLower` (> _returnvalue_z 0.0))
      (bind (_direction _lower_z _xy___rotator _upper_z) (`Timeline|GunFlyToPlayerController` :!via `PlayFromStart`)
        (:`Update`
          (set `self.Location Offset` (`KismetMathLibrary.MakeVector` _returnvalue_x_2 _returnvalue_y_2 _returnvalue_z_2))
          (`self.K2_SetActorLocation` (+ (`self.Original Location`) (`KismetMathLibrary.MakeVector` (* _location_offset_x _xy___rotator) (* _location_offset_y _xy___rotator) (`KismetMathLibrary.SelectFloat` (* _location_offset_z _lower_z) (* _location_offset_z _upper_z) (`self.isLower`)))) false true)
          (`self.K2_SetActorRotation` (`KismetMathLibrary.MakeRotator` (`KismetMathLibrary.MapRangeClamped` _xy___rotator 0.0 1.0 _originalrotation_roll) (`KismetMathLibrary.MapRangeClamped` _xy___rotator 0.0 1.0 _originalrotation_pitch 30.0) (`KismetMathLibrary.MapRangeClamped` _xy___rotator 0.0 1.0 _originalrotation_yaw 180.0)) true))
        (:`Finished`
          (`PrimitiveComponent.SetSimulatePhysics` (`self.Body`) true)
          (`/Game/PLK_MR/Blueprints/BP_VRPawn.CatchGun` (cast `/Game/PLK_MR/Blueprints/BP_VRPawn` (`ActorComponent.GetOwner` ControllerRef) :!pure true) (`self.GrabComponent`) HandType))))))

(event `ResetGun`
  (bind _shooting_point (`self.Shooting Point`))
  (bind _shooting_point_2 (`self.Shooting Point`))
  ;[1 1 1] Gun interaction
  (switch `/Game/PLK_MR/Blueprints/Enum/Enum_GunType` (`self.GunType`)
    (:`NewEnumerator0`
      (goto _label_2 :!via `Reset`))
    (:`NewEnumerator1`
      (goto _label_3 :!via `Reset`))
    (:`NewEnumerator2`
      (goto _label_2 :!via `Reset`))
    (:`NewEnumerator4`
      (`self.Remove Laser`))))

(event `Shooting`
  (params (HandType :type "EControllerHand Enum" :default "Left"))
  (bind _shooting_point (`self.Shooting Point`))
  (bind _shooting_point_2 (`self.Shooting Point`))
  (bind _shooting_point_3 (`self.Shooting Point`))
  (bind _shooting_point_4 (`self.Shooting Point`))
  (bind _spline (`self.Spline`))
  (bind _returnvalue (`SceneComponent.K2_GetComponentLocation` _shooting_point_3))
  (bind _returnvalue_2 (+ _returnvalue (* (`SceneComponent.GetForwardVector` _shooting_point_3) 10000.0)))
  ;[1 1 1] Gun interaction
  (switch `/Game/PLK_MR/Blueprints/Enum/Enum_GunType` (`self.GunType`)
    (:`NewEnumerator0`
      (if (or (> (`self.Ammo`) 0) (`/Game/PLK_MR/GameModes/SharedSpaces/BP_PLKPlayerState.GodMode` (`/Game/PLK_MR/Library/BP_FunctionLibrary.GetOwningPlayerState`))) :!label _label
        (`/Engine/EditorBlueprintResources/StandardMacros.DoOnce` false :!label _label_2
          (:`Completed`
            (`|SpawnActorFromClass` "/Game/PLK_MR/Blueprints/BP_Bullet.BP_Bullet_C" (`KismetMathLibrary.MakeTransform` (`SceneComponent.K2_GetComponentLocation` _shooting_point_2) (`SceneComponent.K2_GetComponentRotation` _shooting_point_2)) "Undefined" "MultiplyWithRoot" null (select `/Game/PLK_MR/Blueprints/Enum/Enum_GunType` (`self.GunType`) :`NewEnumerator0` 5 :`NewEnumerator1` 5 :`NewEnumerator2` 30 :`NewEnumerator3` 20) (`self.GunType`) null)
            (if (not (`/Game/PLK_MR/GameModes/SharedSpaces/BP_PLKPlayerState.GodMode` (`/Game/PLK_MR/Library/BP_FunctionLibrary.GetOwningPlayerState`)))
              (`/Engine/EditorBlueprintResources/StandardMacros.DecrementInt` (`self.Ammo`)
                (:`  `
                  _)))
            (`self.BulletUpdate` HandType)
            (if (<= (`self.Ammo`) 0)
              (`self.SetReloadTimer`))))))
    (:`NewEnumerator1`
      (if (or (> (`self.Ammo`) 0) (`/Game/PLK_MR/GameModes/SharedSpaces/BP_PLKPlayerState.GodMode` (`/Game/PLK_MR/Library/BP_FunctionLibrary.GetOwningPlayerState`)))
        (`/Engine/EditorBlueprintResources/StandardMacros.DoOnce` false :!label _label_3
          (:`Completed`
            (for _ (range 1 9)
              (`|SpawnActorFromClass` "/Game/PLK_MR/Blueprints/BP_Bullet.BP_Bullet_C" (`KismetMathLibrary.MakeTransform` (`SceneComponent.K2_GetComponentLocation` _shooting_point_4) (`/Game/PLK_MR/Library/BP_FunctionLibrary.Get Spray Angle` (`KismetMathLibrary.GetForwardVector` (`SceneComponent.K2_GetComponentRotation` _shooting_point_4)) 7.0)) "Undefined" "MultiplyWithRoot" null (select `/Game/PLK_MR/Blueprints/Enum/Enum_GunType` (`self.GunType`) :`NewEnumerator0` 5 :`NewEnumerator1` 5 :`NewEnumerator2` 30 :`NewEnumerator3` 20) (`self.GunType`) null))
            (if (not (`/Game/PLK_MR/GameModes/SharedSpaces/BP_PLKPlayerState.GodMode` (`/Game/PLK_MR/Library/BP_FunctionLibrary.GetOwningPlayerState`)))
              (bind _result (`/Engine/EditorBlueprintResources/StandardMacros.DecrementInt` (`self.Ammo`))
                (:`  `
                  _)))
            (`self.BulletUpdate` HandType)
            (if (<= _result 0)
              (`self.SetReloadTimer`))))))
    (:`NewEnumerator2`
      (goto _label))
    (:`NewEnumerator3`
      (if (or (> (`self.Ammo`) 0) (`/Game/PLK_MR/GameModes/SharedSpaces/BP_PLKPlayerState.GodMode` (`/Game/PLK_MR/Library/BP_FunctionLibrary.GetOwningPlayerState`)))
        (`/Engine/EditorBlueprintResources/StandardMacros.DoOnce` false :!label _label_4
          (:`Completed`
            (`|SpawnActorFromClass` "/Game/PLK_MR/Blueprints/BP_Bullet.BP_Bullet_C" (`KismetMathLibrary.MakeTransform` (`SceneComponent.K2_GetComponentLocation` _shooting_point) (`SceneComponent.K2_GetComponentRotation` _shooting_point)) "Undefined" "MultiplyWithRoot" null (select `/Game/PLK_MR/Blueprints/Enum/Enum_GunType` (`self.GunType`) :`NewEnumerator0` 5 :`NewEnumerator1` 5 :`NewEnumerator2` 30 :`NewEnumerator3` 20) (`self.GunType`) null)
            (`|ExecutionSequence`
              (:`then_0`
                (`KismetSystemLibrary.Delay` 0.1)
                (goto _label_4 :!via `Reset`))
              (:`then_1`
                (if (not (`/Game/PLK_MR/GameModes/SharedSpaces/BP_PLKPlayerState.GodMode` (`/Game/PLK_MR/Library/BP_FunctionLibrary.GetOwningPlayerState`)))
                  (bind _result_2 (`/Engine/EditorBlueprintResources/StandardMacros.DecrementInt` (`self.Ammo`))
                    (:`  `
                      _)))
                (`self.BulletUpdate` HandType)
                (if (<= _result_2 0)
                  (`self.SetReloadTimer`))))))))
    (:`NewEnumerator4`
      (`SceneComponent.SetVisibility` (`self.SplineMesh`) false false)
      (bind _outhit (`KismetSystemLibrary.SphereTraceSingle` :`Start` _returnvalue :`End` _returnvalue_2 :`Radius` 3.0 :`TraceChannel` "TraceTypeQuery5" :`TraceColor` (struct :`R` 1.0 :`G` 1.0 :`B` 1.0 :`A` 1.0) :`DrawTime` 0.0))
      (if (`GameplayStatics.BreakHitResult` _outhit)
        (`SplineComponent.SetLocationAtSplinePoint` _spline 1 (`.Location` (`GameplayStatics.BreakHitResult` _outhit)) "World" true)
        (else
          (`SplineComponent.SetLocationAtSplinePoint` _spline 1 _returnvalue_2 "World" true)))
      (`self.UpdateSplineMesh`)
      (`|ExecutionSequence`
        (:`then_0`
          (bind _asbp_base_enemy (cast `/Game/PLK_MR/Blueprints/Enemy/BP_BaseEnemy` (`.HitActor` (`GameplayStatics.BreakHitResult` _outhit)))
            (:`then`
              (`/Game/PLK_MR/Blueprints/Enemy/BP_BaseEnemy.Damaged` _asbp_base_enemy 20 true))
            (:`CastFailed`
              (bind _asbp_boss (cast `/Game/PLK_MR/Blueprints/BP_Boss` (`.HitActor` (`GameplayStatics.BreakHitResult` _outhit)))
                (:`then`
                  (`/Engine/EditorBlueprintResources/StandardMacros.DoOnce` false :!label _label_5
                    (:`Completed`
                      (`|ExecutionSequence`
                        (:`then_0`
                          (if (`ActorComponent.ComponentHasTag` (`.HitComponent` (`GameplayStatics.BreakHitResult` _outhit)) "Ans1")
                            (`/Game/PLK_MR/Blueprints/BP_Boss.HitWeakpoint` _asbp_boss 1)
                            (elif (`ActorComponent.ComponentHasTag` (`.HitComponent` (`GameplayStatics.BreakHitResult` _outhit)) "Ans2")
                              (`/Game/PLK_MR/Blueprints/BP_Boss.HitWeakpoint` _asbp_boss 2)
                              (elif (`ActorComponent.ComponentHasTag` (`.HitComponent` (`GameplayStatics.BreakHitResult` _outhit)) "Ans3")
                                (`/Game/PLK_MR/Blueprints/BP_Boss.HitWeakpoint` _asbp_boss 3)))))
                        (:`then_1`
                          (`KismetSystemLibrary.Delay` 0.3)
                          (goto _label_5 :!via `Reset`))))))
                (:`CastFailed`
                  (bind _asbp_question_answer_between_game (cast `/Game/PLK_MR/Blueprints/Widget/BP_QuestionAnswerBetweenGame` (`.HitActor` (`GameplayStatics.BreakHitResult` _outhit))))
                  (`/Game/PLK_MR/Blueprints/Widget/BP_QuestionAnswerBetweenGame.LaserTracked` _asbp_question_answer_between_game))))))
        (:`then_1`
          (`self.LaserSound`
            (:`then`)
            (:`else`
              (bind _returnvalue_3 (`GameplayStatics.SpawnSoundAtLocation` "/Game/PLK_MR/Blueprints/Sound/Laser.Laser" (`self.K2_GetActorLocation`) (struct) 1.0 1.0 0.0 "/Game/PLK_MR/Blueprints/Sound/3Dsound.3Dsound" null))
              (set `self.LaserSound` _returnvalue_3)
              (`ActorComponent.Activate` (`self.NS_Gunbeam`) true))))))))

(event `BulletUpdate`
  (params (HandType :type "EControllerHand Enum" :default "Left"))
  ;[1 1 1] Bullet Text update
  (`self.SetAmmoText`)
  (`/Game/PLK_MR/Blueprints/BP_VRPawn.PlayHapticEffect` (`/Game/PLK_MR/Library/BP_FunctionLibrary.Get VR Pawn`) HandType)
  (`GameplayStatics.PlaySoundAtLocation` (select `/Game/PLK_MR/Blueprints/Enum/Enum_GunType` (`self.GunType`) :`NewEnumerator5` "/Game/PLK_MR/Blueprints/Sound/HandGunSFX.HandGunSFX" :`NewEnumerator0` "/Game/PLK_MR/Blueprints/Sound/HandGunSFX.HandGunSFX" :`NewEnumerator1` "/Game/PLK_MR/Blueprints/Sound/HandGunSFX.HandGunSFX" :`NewEnumerator2` "/Game/PLK_MR/Blueprints/Sound/HandGunSFX.HandGunSFX" :`NewEnumerator3` "/Game/PLK_MR/Blueprints/Sound/HandGunSFX.HandGunSFX" :`NewEnumerator4` "/Game/PLK_MR/Blueprints/Sound/HandGunSFX.HandGunSFX" :!type "SoundBase Object Reference") (`SceneComponent.K2_GetComponentLocation` (`self.Shooting Point`)) (struct) 1.0 1.0 0.0 "/Game/PLK_MR/Blueprints/Sound/3Dsound.3Dsound" null null null)
  (`ActorComponent.Activate` (`self.N_BulletShoot`) true))

(event `Destroy`
  (`|ExecutionSequence`
    (:`then_0`
      (bind _lasersound (`self.LaserSound`)
        (:`then`
          (`AudioComponent.Stop` _lasersound)
          (`ActorComponent.K2_DestroyComponent` _lasersound))
        (:`else`)))
    (:`then_1`
      (`self.K2_DestroyActor`))))

(event `Remove Laser`
  (bind _lasersound (`self.LaserSound`))
  (bind _spline (`self.Spline`))
  ;[1 1 1] Remove Laser
  (`SplineComponent.SetLocationAtSplinePoint` _spline 1 (`SplineComponent.GetLocationAtSplinePoint` _spline 0 "World") "World" true)
  (`self.UpdateSplineMesh`)
  (`AudioComponent.Stop` _lasersound)
  (`ActorComponent.K2_DestroyComponent` _lasersound)
  (`ActorComponent.Deactivate` (`self.NS_Gunbeam`)))

(event `ChangeOverlayMaterial`
  (params (bIsActive :type Boolean))
  (`MeshComponent.SetOverlayMaterial` (`self.Body`) (select `bool` bIsActive :`true` "/Game/PLK_MR/Materials/M_HighLight_Inst.M_HighLight_Inst" :!type "MaterialInterface Object Reference")))

(event `SetReloadTimer`
  ;[1 1 1] Gun reload
  (if (`KismetSystemLibrary.K2_IsTimerActiveHandle` (`self.ReloadTimer`))
    _
    (elif (not (`/Game/PLK_MR/GameModes/SharedSpaces/BP_PLKPlayerState.GodMode` (`/Game/PLK_MR/Library/BP_FunctionLibrary.GetOwningPlayerState`)))
      (set `self.Ammo` 0)
      (`self.SetAmmoText`)
      (bind _returnvalue (`KismetSystemLibrary.K2_SetTimer` null "ReloadGun" (`BlueprintMapLibrary.Map_Find` (`self.ReloadTime`) (`self.GunType`))))
      (set `self.ReloadTimer` _returnvalue)
      (`GameplayStatics.PlaySoundAtLocation` "/Game/PLK_MR/Blueprints/Sound/StartReload.StartReload" (`self.K2_GetActorLocation`) (struct) 1.0 1.0 0.0 "/Game/PLK_MR/Blueprints/Sound/3Dsound.3Dsound" null null null))))

(event `MoveTrigger`
  (params (Value :type "Float (double-precision)"))
  ;[1 1 1] Trigger Moving
  (switch `/Game/PLK_MR/Blueprints/Enum/Enum_GunType` (`self.GunType`)
    (:`NewEnumerator5`
      (`SceneComponent.K2_SetRelativeLocation` (`self.Gun_1_Cube_009`) (`KismetMathLibrary.MakeVector` 0.0 (`KismetMathLibrary.MapRangeClamped` Value 0.0 1.0 0.0 -50.0)) false true :!label _label_6))
    (:`NewEnumerator0`
      (goto _label_6))
    (:`NewEnumerator1`
      (`SceneComponent.K2_SetRelativeRotation` (`self.Gun_1_Cube_009`) (`KismetMathLibrary.MakeRotator` (`KismetMathLibrary.MapRangeClamped` Value 0.0 1.0 0.0 30.0)) false true))
    (:`NewEnumerator2`
      (`SceneComponent.K2_SetRelativeRotation` (`self.Gun_1_Cube_009`) (`KismetMathLibrary.MakeRotator` (`KismetMathLibrary.MapRangeClamped` Value 0.0 1.0 0.0 30.0)) false true))
    (:`NewEnumerator3`
      (`SceneComponent.K2_SetRelativeLocation` (`self.Gun_1_Cube_009`) (`KismetMathLibrary.MakeVector` 0.0 (`KismetMathLibrary.MapRangeClamped` Value 0.0 1.0 0.0 -2.0)) false true))
    (:`NewEnumerator4`
      (`SceneComponent.K2_SetRelativeLocation` (`self.Gun_1_Cube_009`) (`KismetMathLibrary.MakeVector` 0.0 (`KismetMathLibrary.MapRangeClamped` Value 0.0 1.0 0.0 -10.0)) false true))))

(fn `DistanceDetecter`
  (params (Distance :type "Float (double-precision)"))
  (returns (`PlayerInDistance?` :type Boolean) (ActualDistance :type "Float (double-precision)"))
  (bind (_returnvalue_x _returnvalue_y) (`KismetMathLibrary.BreakVector` (`self.K2_GetActorLocation`)))
  (bind (_returnvalue_x_2 _returnvalue_y_2) (`KismetMathLibrary.BreakVector` (`SceneComponent.K2_GetComponentLocation` (`/Game/PLK_MR/Blueprints/BP_VRPawn.Camera` (`/Game/PLK_MR/Library/BP_FunctionLibrary.Get VR Pawn`)))))
  (bind _returnvalue (`KismetMathLibrary.Vector_Distance` (`KismetMathLibrary.MakeVector` _returnvalue_x _returnvalue_y) (`KismetMathLibrary.MakeVector` _returnvalue_x_2 _returnvalue_y_2)))
  (return (<= _returnvalue Distance) _returnvalue))

(fn `ReloadGun`
  (set `self.Ammo` (`self.MaxAmmo`))
  (`self.SetAmmoText`)
  (`GameplayStatics.PlaySoundAtLocation` "/Game/PLK_MR/Blueprints/Sound/EndReload.EndReload" (`self.K2_GetActorLocation`) (struct) 1.0 1.0 0.0 "/Game/PLK_MR/Blueprints/Sound/3Dsound.3Dsound" null null null))

(fn `SetAmmoText`
  (`/Game/PLK_MR/Blueprints/Widget/WBP_BulletCounter.SetText` (cast `/Game/PLK_MR/Blueprints/Widget/WBP_BulletCounter` (`WidgetComponent.GetWidget` (`self.BulletWidget`)) :!pure true) (`|FormatText` "{Ammo}/{MaxAmmo}" (`self.Ammo`) (`self.MaxAmmo`))))

(fn `UpdateSplineMesh`
  (bind _spline (`self.Spline`))
  (bind (_location _tangent) (`SplineComponent.GetLocationAndTangentAtSplinePoint` _spline 1 "Local"))
  (bind (_location_2 _tangent_2) (`SplineComponent.GetLocationAndTangentAtSplinePoint` _spline 0 "Local"))
  (`SplineMeshComponent.SetStartAndEnd` (`self.SplineMesh`) _location_2 _tangent_2 _location _tangent true))

(fn `UserConstructionScript`)