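; Blueprint function library of shared helpers for the PLK mixed-reality game: room persistence, player lookups, weapon spread and level state.
; Save and load use named BP_RoomSaveGame slots to store BP_Room wall transforms and return them with a success flag.
; Getters resolve player 0's VR pawn and player state, while spray angle picks a random direction within a cone.
; Level setter writes to that player state, then notifies GS_PLK.
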(fn `Get Spray Angle`
  (params (MuzzleDirection :type "Vector Structure") (MaxAngle :type "Float (double-precision)"))
  (returns (ShotRotation :type "Rotator Structure"))
  (return (`KismetMathLibrary.MakeRotFromX` (`KismetMathLibrary.RandomUnitVectorInConeInDegrees` MuzzleDirection MaxAngle))))

(fn `Get VR Pawn`
  (returns (PlayerPawn :type "/Game/PLK_MR/Blueprints/BP_VRPawn Object Reference"))
  (bind _asbp_vrpawn (cast `/Game/PLK_MR/Blueprints/BP_VRPawn` (`GameplayStatics.GetPlayerPawn` null)))
  (return _asbp_vrpawn))

(fn `GetCurrentLevels`
  (params (Levels :type "/Game/PLK_MR/Blueprints/Enum/Enum_GameLevels Enum" :default "NewEnumerator6"))
  (returns (CurrentLevels :type "/Game/PLK_MR/Blueprints/Enum/Enum_GameLevels Enum") (`IsMatch?` :type Boolean))
  (bind _level (`/Game/PLK_MR/GameModes/SharedSpaces/BP_PLKPlayerState.Level` (`self.GetOwningPlayerState` null)))
  (return _level (`|EnumEquality` Levels _level)))

(fn `GetOwningPlayerState`
  (returns (PlayerState :type "/Game/PLK_MR/GameModes/SharedSpaces/BP_PLKPlayerState Object Reference"))
  (bind _asbp_plkplayer_state (cast `/Game/PLK_MR/GameModes/SharedSpaces/BP_PLKPlayerState` (`Pawn.PlayerState` (`GameplayStatics.GetPlayerPawn` null)))
    (:`then`
      (return _asbp_plkplayer_state))
    (:`CastFailed`
      (return null))))

(fn `Load Game`
  (params (Slot :type String))
  (returns (`Success?` :type Boolean) (WallsTrans :type "Array of Float (double-precision)"))
  (locals (Success :type Boolean :default false) (`Walls Trans` :type "Array of Float (double-precision)"))
  (bind _returnvalue (`GameplayStatics.DoesSaveGameExist` Slot))
  (`|ExecutionSequence`
    (:`then_0`
      (if _returnvalue
        (set `local.Success` true)
        (bind _returnvalue_2 (`GameplayStatics.LoadGameFromSlot` Slot))
        (bind _asbp_room_save_game (cast `/Game/PLK_MR/Blueprints/SaveGame/BP_RoomSaveGame` _returnvalue_2))
        (set `local.Walls Trans` (`/Game/PLK_MR/Blueprints/SaveGame/BP_RoomSaveGame.Walls_Details` _asbp_room_save_game))))
    (:`then_1`
      (return (`local.Success`) (`local.Walls Trans`)))))

(fn `NewFunction`)

(fn `Save Game`
  (params (Slot :type String))
  (locals (SaveREF :type "SaveGame Object Reference"))
  (bind _returnvalue (`GameplayStatics.DoesSaveGameExist` Slot))
  (if _returnvalue
    (bind _returnvalue_2 (`GameplayStatics.LoadGameFromSlot` Slot))
    (set `local.SaveREF` _returnvalue_2)
    (else
      (bind _returnvalue_3 (`GameplayStatics.CreateSaveGameObject` "/Game/PLK_MR/Blueprints/SaveGame/BP_RoomSaveGame.BP_RoomSaveGame_C"))
      (bind _output_get (set `local.SaveREF` _returnvalue_3))))
  (bind _asbp_room_save_game (cast `/Game/PLK_MR/Blueprints/SaveGame/BP_RoomSaveGame` _output_get))
  (bind _returnvalue_4 (`GameplayStatics.GetActorOfClass` null "/Game/PLK_MR/Blueprints/BP_Room.BP_Room_C"))
  (bind _wallstrans (`/Game/PLK_MR/Blueprints/BP_Room.GetAllWallsTrans` _returnvalue_4))
  (`/Game/PLK_MR/Blueprints/SaveGame/BP_RoomSaveGame.CreateSaveData` _asbp_room_save_game _wallstrans)
  (`GameplayStatics.SaveGameToSlot` (`local.SaveREF`) Slot))

(fn `SetGameLevels`
  (params (Level :type "/Game/PLK_MR/Blueprints/Enum/Enum_GameLevels Enum" :default "NewEnumerator6"))
  (returns (Levels :type "/Game/PLK_MR/Blueprints/Enum/Enum_GameLevels Enum"))
  (bind _output_get (set `/Game/PLK_MR/GameModes/SharedSpaces/BP_PLKPlayerState.Level` Level (`self.GetOwningPlayerState` null)))
  (`/Game/PLK_MR/GameModes/SharedSpaces/GS_PLK.GS_LevelsUpdate` (cast `/Game/PLK_MR/GameModes/SharedSpaces/GS_PLK` (`GameplayStatics.GetGameState` null) :!pure true) _output_get)
  (return Level))